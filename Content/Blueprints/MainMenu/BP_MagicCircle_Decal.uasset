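; Main menu magic circle decal actor that spins its MagicCircle component around its local roll axis.
; Each tick, UpdateTimeTick accumulates delta seconds into Time, wrapped at two pi.
; Tick then adds Time multiplied by RotationSpeed as a roll increment, so the per-frame spin ramps up until Time wraps and is not scaled by frame time.
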(event `self.ReceiveTick`
  (params (DeltaSeconds :type "Float (single-precision)"))
  (`self.UpdateTimeTick` DeltaSeconds)
  (`SceneComponent.K2_AddLocalRotation` (`self.Magic Circle`) (`KismetMathLibrary.MakeRotator` (* (`self.Time`) (`self.RotationSpeed`))) false false))

(fn `UpdateTimeTick`
  (params (`Delta Seconds` :type "Float (double-precision)"))
  (set `self.Time` (`KismetMathLibrary.FMod` (+ `Delta Seconds` (`self.Time`)) (* (`KismetMathLibrary.GetPI`) 2.0))))

(fn `UserConstructionScript`)