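; BP_Character_MainMenu is the character shown in the main menu, which also sets up that menu.
; On BeginPlay it plays the menu music, adds WBP_MainMenu to the viewport and switches to UI-only input with a visible cursor.
; Each tick bobs its Fireball vertically along a sine wave around its start location, using a time value wrapped at two pi.
; The music component is destroyed along with the actor.
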(event `self.ReceiveBeginPlay`
  (set `self.FireballInitialLoctaion` (`SceneComponent.K2_GetComponentLocation` (`self.Fireball`)))
  (bind _returnvalue (`GameplayStatics.SpawnSound2D` "/Game/Assets/Sounds/Music/Music_MainMenu.Music_MainMenu" 1.0 1.0 0.0 null))
  (set `self.MenuBGM` _returnvalue)
  (bind _returnvalue_2 (`|CreateWidget` "/Game/Blueprints/UI/MainMenu/WBP_MainMenu.WBP_MainMenu_C"))
  (`UserWidget.AddToViewport` _returnvalue_2 0)
  (set `self.MainMenuWidget` _returnvalue_2)
  (`WidgetBlueprintLibrary.SetInputMode_UIOnlyEx` (`GameplayStatics.GetPlayerController` 0) null)
  (set `PlayerController.bShowMouseCursor` true (`GameplayStatics.GetPlayerController` 0)))

(event `self.ReceiveTick`
  (params (DeltaSeconds :type "Float (single-precision)"))
  (`self.UpdateTimeTick` DeltaSeconds)
  (`SceneComponent.K2_SetWorldLocation` (`self.Fireball`) (+ (`self.FireballInitialLoctaion`) (`KismetMathLibrary.MakeVector` 0.0 0.0 (* (`KismetMathLibrary.Sin` (`self.Time`)) (`self.FireballLevitationMagnitude`)))) false false))

(event `self.ReceiveDestroyed`
  (`ActorComponent.K2_DestroyComponent` (`self.MenuBGM`)))

(fn `UpdateTimeTick`
  (params (A :type "Float (double-precision)"))
  (set `self.Time` (`KismetMathLibrary.FMod` (+ A (`self.Time`)) (* (`KismetMathLibrary.GetPI`) 2.0))))

(fn `UserConstructionScript`)