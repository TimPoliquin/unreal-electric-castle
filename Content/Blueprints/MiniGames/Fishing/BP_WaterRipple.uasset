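; Water ripple effect actor for the fishing minigame, shown and hidden on demand.
; PlayRipple makes the root and its children visible, then plays the RippleSequence animation either once or looping indefinitely.
; StopRipple stops the sequence and hides the hierarchy; a one-shot play has no automatic hide in this graph.
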(event `self.PlayRipple`
  (params (bLoop :type Boolean))
  (bind _ripple_sequence (`self.Ripple Sequence`))
  (`SceneComponent.SetVisibility` (`self.DefaultSceneRoot`) true true)
  (if bLoop
    (`MovieSceneSequencePlayer.PlayLooping` (`ActorSequenceComponent.SequencePlayer` _ripple_sequence) -1)
    (else
      (`ActorSequenceComponent.PlaySequence` _ripple_sequence))))

(event `self.StopRipple`
  (`ActorSequenceComponent.StopSequence` (`self.Ripple Sequence`))
  (`SceneComponent.SetVisibility` (`self.DefaultSceneRoot`) false true))

(fn `UserConstructionScript`)