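; BP_Fishing_POI is a point of interest that runs the fishing minigame for a player.
; StartFishing launches a GoFishing async task and routes each stage delegate, from player in position through cast, lure, bite and reel, to the matching Trigger call.
; The task ends when the fish flees or is caught.
; TriggerFishReel extends the parent's behavior by triggering the catch after a short fixed delay.
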(event `self.StartFishing`
  (params (Player :type "Actor Object Reference"))
  (`parent.StartFishing` Player)
  (bind (_asynctaskproxy _fishingactor _catch) (`FishingBlueprintNode.GoFishing` Player (`self.MakeGoFishingParams`))
    (:`OnPlayerInPositionDelegate`
      (`self.TriggerEquipFishingRod` null))
    (:`OnFishingRodEquippedDelegate`
      (`self.TriggerFishingCast` null))
    (:`OnFishingRodCastDelegate`
      (`self.TriggerBobSplashEffect`))
    (:`OnFishingLuredDelegate`
      (`self.TriggerFishInterested` null _asynctaskproxy))
    (:`OnFishingBiteDelegate`
      (`self.TriggerFishBite` null))
    (:`OnFishingFishHasFledDelegate`
      (`self.TriggerFishFled` null)
      (`FishingBlueprintNode.End` _asynctaskproxy))
    (:`OnFishingFishReelingDelegate`
      (`self.TriggerFishReel` null _asynctaskproxy))
    (:`OnFishingFishCaughtDelegate`
      (`self.TriggerFishCaught` null _catch)
      (`FishingBlueprintNode.End` _asynctaskproxy))))

(event `self.TriggerFishReel`
  (params (Player :type "Actor Object Reference") (FishingTask :type "FishingBlueprintNode Object Reference"))
  (`parent.TriggerFishReel` Player FishingTask)
  (`KismetSystemLibrary.Delay` 1.0)
  (`self.TriggerFishCatch` Player FishingTask))

(fn `UserConstructionScript`)