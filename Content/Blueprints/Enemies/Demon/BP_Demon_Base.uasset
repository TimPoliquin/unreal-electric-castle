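; Base Blueprint for Demon enemies that declares the combat sockets on the character mesh.
; The RegisterSockets override calls its parent, then registers left hand, right hand and tail mesh sockets with the socket manager component under Combat.Socket gameplay tags.
; It adds no other logic: BeginPlay, overlap and Tick are disabled stubs, and the construction script only calls its parent.
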(event `self.RegisterSockets`
  (params (InSocketManagerComponent :type "SocketManagerComponent Object Reference"))
  (`parent.RegisterSockets` InSocketManagerComponent)
  (`SocketManagerComponent.RegisterSocket` InSocketManagerComponent (`self.Mesh`) (struct :`TagName` "Combat.Socket.LeftHand") "LeftHand_Socket")
  (`SocketManagerComponent.RegisterSocket` InSocketManagerComponent (`self.Mesh`) (struct :`TagName` "Combat.Socket.RightHand") "RightHand_Socket")
  (`SocketManagerComponent.RegisterSocket` InSocketManagerComponent (`self.Mesh`) (struct :`TagName` "Combat.Socket.Tail") "TailSocket"))

(fn `UserConstructionScript`
  (`parent.UserConstructionScript`))