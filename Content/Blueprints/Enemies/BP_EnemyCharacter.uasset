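; BP_EnemyCharacter is the enemy character Blueprint, adding an alert meter, stagger and hit feedback to its parent class.
; On BeginPlay it constructs an MVVM AI alert view model bound to itself and passes it to the alert meter widget.
; Significance changes toggle that widget's visibility, and local death hides it.
; Stagger applies a gameplay effect, while damage plays a timeline driving the HitFlash parameter on dynamic materials.
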(event `self.ReceiveBeginPlay`
  (`parent.ReceiveBeginPlay`)
  (`self.Initialize View Models`)
  (`self.Initialize Widgets`))

(event `CombatInterface.Stagger`
  (`ElectricCastleAbilitySystemLibrary.ApplyBasicGameplayEffect` self "/Game/Blueprints/AbilitySystem/GameplayEffects/Status/GE_Staggered.GE_Staggered_C"))

(event `self.HandleDeathLocal`
  (`parent.HandleDeathLocal`)
  (`SceneComponent.SetVisibility` (`self.Alert Level Widget`) false true))

(event `self.EnterSignificance_PartiallySignificant`
  (`parent.EnterSignificance_PartiallySignificant`)
  (`SceneComponent.SetVisibility` (`self.Alert Level Widget`) true false))

(event `self.EnterSignificance_FullySignificant`
  (`parent.EnterSignificance_FullySignificant`)
  (`SceneComponent.SetVisibility` (`self.Alert Level Widget`) true false))

(event `self.EnterSignificance_Insignificant`
  (`parent.EnterSignificance_Insignificant`)
  (`SceneComponent.SetVisibility` (`self.Alert Level Widget`) false false))

(event `self.HandleTakeDamage_HitFlash`
  (`parent.HandleTakeDamage_HitFlash`)
  (bind (_direction _alpha) (`Timeline|HitFlash Timeline` :!via `PlayFromStart`)
    (:`Update`
      (for _array_element (`self.DynamicMeshMaterials`)
        (`MaterialInstanceDynamic.SetScalarParameterValue` _array_element "HitFlash" _alpha)))))

(fn `Initialize View Models`
  (`|ExecutionSequence`
    (:`then_0`
      ; Setup AI Alert Model
      (bind _returnvalue (`|GenericCreateObject` "/Game/Blueprints/UI/AI/ViewModel/MVVM_AI_Alert.MVVM_AI_Alert_C"))
      (bind _output_get (set `self.MVVM_AI_Alert` _returnvalue))
      (`/Engine/EditorBlueprintResources/StandardMacros.IsValid` _output_get
        (:`Is Valid`
          (`/Game/Blueprints/UI/AI/ViewModel/MVVM_AI_Alert.Initialize Dependencies` _output_get self))))))

(fn `Initialize Widgets`
  (`|ExecutionSequence`
    (:`then_0`
      ; Initialize Alert Level Widget
      (bind _aswbp_ai_alert_meter (cast `/Game/Blueprints/UI/AI/WBP_AI_AlertMeter` (`WidgetComponent.GetWidget` (`self.Alert Level Widget`))))
      (`/Engine/EditorBlueprintResources/StandardMacros.IsValid` _aswbp_ai_alert_meter
        (:`Is Valid`
          (`/Game/Blueprints/UI/AI/WBP_AI_AlertMeter.Initialize View Model` _aswbp_ai_alert_meter (`self.MVVM_AI_Alert`)))))))

(fn `UserConstructionScript`)