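; Base Blueprint for goblin enemies that maps combat socket tags to sockets on the goblin mesh.
; On RegisterSockets it registers left hand, right hand and stagger-stars effect sockets with the supplied socket manager component.
; It registers the same mesh sockets with the weapon child actor's socket manager, fetched by message call, when that is valid.
; BeginPlay, overlap, Tick and construction script add no logic of their own.
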(event `self.RegisterSockets`
  (params (InSocketManagerComponent :type "SocketManagerComponent Object Reference"))
  (`self.Register Sockets to Socket Manager` InSocketManagerComponent)
  (bind _returnvalue (message `SocketManagerActor.GetSocketManagerComponent` (`ChildActorComponent.ChildActor` (`self.WeaponChildActorComponent`))))
  (`/Engine/EditorBlueprintResources/StandardMacros.IsValid` _returnvalue
    (:`Is Valid`
      (`self.Register Sockets to Socket Manager` _returnvalue))))

(event `Register Sockets to Socket Manager`
  (params (`In Socket Manager Component` :type "SocketManagerComponent Object Reference"))
  (`SocketManagerComponent.RegisterSocket` `In Socket Manager Component` (`self.Mesh`) (struct :`TagName` "Combat.Socket.LeftHand") "WeaponHandSocket")
  (`SocketManagerComponent.RegisterSocket` `In Socket Manager Component` (`self.Mesh`) (struct :`TagName` "Combat.Socket.RightHand") "RightHand_Socket")
  (`SocketManagerComponent.RegisterSocket` `In Socket Manager Component` (`self.Mesh`) (struct :`TagName` "Combat.Socket.Effect.Stagger") "Effect.StaggerStars"))

(fn `UserConstructionScript`
  (`parent.UserConstructionScript`))