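; Goblin slingshot weapon Blueprint that drives the slingshot's own animation Blueprint.
; On BeginPlay it caches the mesh's ABP_Slingshot instance for later calls.
; SetIsHoldingPouch forwards the pouch-held flag to that anim instance, and Fire clears the flag and plays the slingshot attack montage.
; The file spawns no projectile; it handles only the weapon's animation.
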(event `self.ReceiveBeginPlay`
  (bind _asabp_slingshot (cast `/Game/Blueprints/Enemies/Goblins/Slingshot/ABP_Slingshot` (`SkeletalMeshComponent.GetAnimInstance` (`self.MeshComponent`))))
  (set `self.Animation Blueprint` _asabp_slingshot))

(event `Fire`
  (`self.Animation Blueprint`
    (:`then`
      (`self.Set Is Holding Pouch` false)
      (`AnimInstance.Montage_Play` (`self.Animation Blueprint`) "/Game/Assets/Enemies/GoblinToon/Slingshot/Centered/AM_Slingshot_Attack.AM_Slingshot_Attack" 1.0 "MontageLength" 0.0 true))
    (:`else`)))

(event `Set Is Holding Pouch`
  (params (`Is Holding Pouch` :type Boolean))
  (bind _animation_blueprint (`self.Animation Blueprint`)
    (:`then`
      (set `/Game/Blueprints/Enemies/Goblins/Slingshot/ABP_Slingshot.IsHoldingPouch` `Is Holding Pouch` _animation_blueprint))
    (:`else`)))

(fn `UserConstructionScript`)