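; Base actor for state-shift level assets, exposing its StateShift component and defining reaction events for visibility and collision changes.
; Show and hide reactions set actor visibility, and fade-in and fade-out default to those instant toggles.
; Collision enable and disable are placeholders that log an on-screen error tagged with the object name, so children must implement them.
; The collision-component getter returns nothing here.
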(event `self.StateShiftReaction_Visibility_Show`
  (`StateShiftBlueprintFunctionLibrary.SetActorVisibility` null true))

(event `self.StateShiftReaction_Visibility_Hide`
  (`StateShiftBlueprintFunctionLibrary.SetActorVisibility` null))

(event `self.StateShiftReaction_Collision_Enable`
  (`self.Event LogError` "Must implement StateShiftReaction_Collision_Enable"))

(event `self.StateShiftReaction_Collision_Disable`
  (`self.Event LogError` "Must implement StateShiftReaction_Collision_Disable"))

(event `self.StateShiftReaction_Visibility_FadeOut`
  (`self.StateShiftReaction_Visibility_Hide`))

(event `self.StateShiftReaction_Visibility_FadeIn`
  (`self.StateShiftReaction_Visibility_Show`))

(event `Event LogError`
  (params (D :type String))
  (`KismetSystemLibrary.PrintString` (`KismetStringLibrary.Concat_StrStr` "[" (`KismetSystemLibrary.GetObjectName` self) "] " D) true true (struct :`R` 1.0 :`G` 0.318429 :`A` 1.0) 100.0))

(fn `GetStateShiftCollisionComponent`
  (returns (ReturnValue :type "ShapeComponent Object Reference"))
  (return null))

(fn `GetStateShiftComponent`
  (returns (ReturnValue :type "StateShiftComponent Object Reference"))
  (return (`self.StateShift`)))

(fn `UserConstructionScript`)