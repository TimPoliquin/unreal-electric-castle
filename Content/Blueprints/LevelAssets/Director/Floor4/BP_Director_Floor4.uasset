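; Level director for Floor 4 that runs a horde mode and hands out rewards between rounds.
; After an initial delay it starts rounds through HordeModeComponent, and each completed round grants rewards, then starts the next after a delay if one remains.
; Rewards become spawn params around a RewardSpawn point, then spawn one by one via a recursive delayed event, each attached to a spawn effect that animates it toward its target.
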(event `self.ReceiveBeginPlay`
  (add `HordeModeComponent.OnHordeModeRoundComplete` (`self.HordeModeComponent`) (delegate `OnHoardModeRoundComplete_Event`))
  (`KismetSystemLibrary.Delay` (`self.Initial Delay`))
  (`self.Start Hoard Mode`))

(event `OnHoardModeRoundComplete_Event`
  (params (Payload :type "OnHordeModeRoundCompletePayload Structure (by ref)"))
  (bind (_completedround _nextround _hasnextround _rewards) (break `OnHordeModeRoundCompletePayload` Payload))
  (`self.Grant Rewards` _rewards)
  (if _hasnextround
    (`KismetSystemLibrary.Delay` (`self.Round Delay`))
    (`HordeModeComponent.StartRound` (`self.HordeModeComponent`))))

(event `Start Hoard Mode`
  (`HordeModeComponent.StartRound` (`self.HordeModeComponent`)))

(event `Grant Rewards`
  (params (`Rewards Config` :type "Array of HordeRoundRewards Structure"))
  (bind _returnvalue (`HordeModeComponent.ConvertRewardsToSpawnParams` (`self.HordeModeComponent`) (`self.K2_GetActorLocation` (`ChildActorComponent.ChildActor` (`self.Reward Spawn`))) 150.0 `Rewards Config`))
  (`self.Spawn Reward` _returnvalue))

(event `Spawn Reward`
  (params (`Spawn Params` :type "Array of AuraSpawnParams Structure"))
  (bind _returnvalue (`ElectricCastleSpawnBlueprintLibrary.SafePop` `Spawn Params`))
  (bind (_spawnclass _spawntransform) (break `AuraSpawnParams` _returnvalue))
  (bind _returnvalue_2 (`|SpawnActorFromClass` _spawnclass (`self.GetTransform` (`ChildActorComponent.ChildActor` (`self.Reward Spawn`))) "AdjustIfPossibleButAlwaysSpawn" "MultiplyWithRoot" null null))
  (`self.Animate Reward Spawn` _returnvalue_2 _spawntransform)
  (if (`KismetArrayLibrary.Array_IsNotEmpty` `Spawn Params`)
    (`KismetSystemLibrary.Delay` 0.25)
    (`self.Spawn Reward` `Spawn Params`)))

(event `Animate Reward Spawn`
  (params (Reward :type "Actor Object Reference") (`Target Transform` :type "Transform Structure"))
  (bind _returnvalue (`self.GetTransform` Reward))
  (bind _returnvalue_2 (`|SpawnActorFromClass` "/Game/Blueprints/Items/Animation/BP_SpawnEffect.BP_SpawnEffect_C" _returnvalue "AlwaysSpawn" "MultiplyWithRoot" null null))
  (`self.K2_AttachToActor` Reward _returnvalue_2 "None" "SnapToTarget" "SnapToTarget" "SnapToTarget" true)
  (message `SpawnEffectInterface.PlaySpawnEffect` _returnvalue_2 (make `AuraSpawnEffectParams` _returnvalue `Target Transform` 100.0)))

(fn `Generate Transforms from Rewards Config`
  (params (Rewards :type "Array of HordeRoundRewards Structure"))
  (returns (`Spawn Transforms` :type "Array of Transform Structure"))
  (return (`ElectricCastleSpawnBlueprintLibrary.GenerateSpawnLocations` (`self.K2_GetActorLocation` (`ChildActorComponent.ChildActor` (`self.Reward Spawn`))) 100.0 (`HordeModeConfig.GetNumberOfRewardsToSpawn` Rewards))))

(fn `UserConstructionScript`)