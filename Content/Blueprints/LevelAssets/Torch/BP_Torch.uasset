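; BP_Torch is a level prop torch that can be lit or extinguished, toggling its Fire and FireSFX components together.
; The Lit variable sets both components' auto-activation in the construction script and is reapplied through SetLit on BeginPlay.
; SetLit routes to Light or Extinguish, which update Lit and activate or deactivate both components.
; An OnTrigger event passes its Activate flag to SetLit, so triggers can switch the torch during play.
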(event `self.ReceiveBeginPlay`
  (`self.Set Lit` (`self.Lit`)))

(event `Light`
  (set `self.Lit` true)
  (`ActorComponent.Activate` (`self.Fire`) false)
  (`ActorComponent.Activate` (`self.FireSFX`) false))

(event `Extinguish`
  (set `self.Lit` false)
  (`ActorComponent.Deactivate` (`self.Fire`))
  (`ActorComponent.Deactivate` (`self.FireSFX`)))

(event `Set Lit`
  (params (`Is Lit` :type Boolean))
  (if `Is Lit`
    (`self.Light`)
    (else
      (`self.Extinguish`))))

(event `/Game/Blueprints/LevelAssets/Button/BI_Triggerable.OnTrigger`
  (params (Activate :type Boolean))
  (`self.Set Lit` Activate))

(fn `UserConstructionScript`
  (`ActorComponent.SetAutoActivate` (`self.Fire`) (`self.Lit`))
  (`ActorComponent.SetAutoActivate` (`self.FireSFX`) (`self.Lit`)))