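; BP_Beacon is a switch-style beacon that lights up when activated and goes dark when reset.
; Activation calls the parent logic, then drives the Glow parameter on a dynamic material instance, either ramped by a timeline or set instantly when Forced.
; It broadcasts activation once full glow is applied or the timeline finishes, and reset zeroes the glow and broadcasts a reset.
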(event `self.ActivateBeacon`
  (params (bForced :type Boolean))
  (`parent.ActivateBeacon` bForced)
  (if bForced
    (`MaterialInstanceDynamic.SetScalarParameterValue` (`self.DynamicMaterialInstance`) "Glow" (`self.Glow Multiplier`))
    (`self.BroadcastOnBeaconActivated`)
    (else
      (bind (_direction _alpha) (`Timeline|Beacon Timeline` :!via `PlayFromStart`)
        (:`Update`
          (`MaterialInstanceDynamic.SetScalarParameterValue` (`self.DynamicMaterialInstance`) "Glow" (* _alpha (`self.Glow Multiplier`))))
        (:`Finished`
          (`self.BroadcastOnBeaconActivated`))))))

(event `SwitchInterface.ResetSwitch`
  (`parent.ResetSwitch`)
  (`MaterialInstanceDynamic.SetScalarParameterValue` (`self.DynamicMaterialInstance`) "Glow" 0.0)
  (`self.BroadcastOnBeaconReset`))

(fn `UserConstructionScript`)