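; BP_Beacon_Crystal is a crystal level prop that glows in response to the state of a referenced Beacon.
; On BeginPlay it creates a dynamic material with its color and vibrance, sets emission to zero, and binds to the Beacon's activated and reset events.
; Activation plays a timeline that animates emission by a glow multiplier, while reset cuts emission instantly, each after checking the Beacon's switch state.
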(event `self.ReceiveBeginPlay`
  (bind _returnvalue (`KismetMaterialLibrary.CreateDynamicMaterialInstance` (`PrimitiveComponent.GetMaterial` (`self.Crystal Mesh`) 0) "Crystal Material"))
  (set `self.Dynamic Material` _returnvalue)
  (`PrimitiveComponent.SetMaterial` (`self.Crystal Mesh`) 0 (`self.Dynamic Material`))
  (`MaterialInstanceDynamic.SetVectorParameterValue` (`self.Dynamic Material`) "Color" (`self.Color`))
  (`MaterialInstanceDynamic.SetScalarParameterValue` (`self.Dynamic Material`) "Vibrance" (`self.Vibrance`))
  (`MaterialInstanceDynamic.SetScalarParameterValue` (`self.Dynamic Material`) "Emission" 0.0)
  (add `Beacon.OnBeaconActivated` (`self.Beacon`) (delegate `OnBeaconActivated_Event`))
  (add `Beacon.OnBeaconReset` (`self.Beacon`) (delegate `OnBeaconReset_Event`)))

(event `OnBeaconActivated_Event`
  (params (Payload :type "OnSwitchStatusChangedPayload Structure (by ref)"))
  (`self.Activate Crystal`))

(event `OnBeaconReset_Event`
  (params (Payload :type "OnSwitchStatusChangedPayload Structure (by ref)"))
  (`self.Deactivate Crystal`))

(event `Activate Crystal`
  (if (`SwitchInterface.IsSwitchActive` (`self.Beacon`))
    (bind (_direction _alpha) (`Timeline|Activate Timeline` :!via `PlayFromStart`)
      (:`Update`
        (`MaterialInstanceDynamic.SetScalarParameterValue` (`self.Dynamic Material`) "Emission" (* _alpha (`self.Glow Multiplier`)))))))

(event `Deactivate Crystal`
  (if (not (`SwitchInterface.IsSwitchActive` (`self.Beacon`)))
    (`MaterialInstanceDynamic.SetScalarParameterValue` (`self.Dynamic Material`) "Emission" 0.0)))

(fn `UserConstructionScript`)