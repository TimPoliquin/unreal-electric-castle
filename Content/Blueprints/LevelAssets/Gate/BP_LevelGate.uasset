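; BP_LevelGate is a level gate blocked by a forcefield that can be permanently unlocked.
; Unlock runs a timeline driving the forcefield material's Alpha, then sets Unlocked, hides the box, disables collision and stops the static sound.
; BeginPlay and LoadActor both initialize from the Unlocked flag, either applying the open state directly or creating the dynamic material.
; ShouldLoadTransform returns false, so loading leaves the transform untouched.
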(event `self.ReceiveBeginPlay`
  (`self.Initialize State`))

(event `SaveInterface.LoadActor`
  (`self.Initialize State`))

(event `LockInterface.Unlock`
  (`self.Forcefield Dynamic Material`
    (:`then`
      (bind (_direction _alpha) (`Timeline|Unlock Timeline` :!via `PlayFromStart`)
        (:`Update`
          (`MaterialInstanceDynamic.SetScalarParameterValue` (`self.Forcefield Dynamic Material`) "Alpha" _alpha))
        (:`Finished`
          (set `self.Unlocked` true :!label _label)
          (`self.Mark Unlocked`))))
    (:`else`
      (goto _label))))

(fn `Initialize Dynamic Materials`
  (bind _forcefield_mesh (`self.Forcefield Mesh`))
  (bind _returnvalue (`PrimitiveComponent.CreateDynamicMaterialInstance` _forcefield_mesh 0 (`PrimitiveComponent.GetMaterial` _forcefield_mesh 0) "Forcefield"))
  (set `self.Forcefield Dynamic Material` _returnvalue))

(fn `Initialize State`
  (if (`self.Unlocked`)
    (`self.Mark Unlocked`)
    (else
      (`self.Initialize Dynamic Materials`))))

(fn `Mark Unlocked`
  (`SceneComponent.SetVisibility` (`self.Box`) false true)
  (`PrimitiveComponent.SetCollisionEnabled` (`self.Box`) "NoCollision")
  (`PrimitiveComponent.SetCollisionEnabled` (`self.Forcefield Mesh`) "NoCollision")
  (`AudioComponent.Stop` (`self.Static Sound`)))

(fn `ShouldLoadTransform`
  (returns (ReturnValue :type Boolean))
  (return false))

(fn `UserConstructionScript`)