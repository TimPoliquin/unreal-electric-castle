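; Interactable point-of-interest actor that a player in Barbarian form can knock down, moving it to a target transform.
; Interaction disables the POI, plays the smash montage on characters and waits for its gameplay event before a Timeline lerps the transform.
; Camera shakes, sounds and pooled Niagara effects mark start and impact.
; While overlapped, it listens for player form changes to re-run the overlap handling.
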(event `Knockdown`
  (params (`Player Actor` :type "Actor Object Reference"))
  (`|ExecutionSequence`
    (:`then_0`
      (set `self.Starting Transform` (`self.GetTransform`))
      (`self.DisablePOI`))
    (:`then_1`
      (message `CombatInterface.UpdateFacingTarget` `Player Actor` (`SceneComponent.K2_GetComponentLocation` (`self.Effect Root`)))
      (bind _ascharacter (cast `Character` `Player Actor`)
        (:`then`
          (`|PlayMontage` (`Character.Mesh` _ascharacter) "/Game/MetaHumans/MHC_Barbarian/Animations/Action/AM_Barbarian_Smash.AM_Barbarian_Smash"
            (:`then`
              (`AbilityAsync_WaitGameplayEvent.WaitGameplayEventToActor` `Player Actor` (struct :`TagName` "Event.Montage.Barbarian.Action.Smash")
                (:`EventReceived`
                  (`self.On Smash Hit`))))))
        (:`CastFailed`
          (`self.On Smash Hit`))))))

(event `On Smash Hit`
  (bind (_sfx _vfx) (`self.Play Start Effects`))
  (bind (_direction _progress) (`Timeline|Timeline`)
    (:`Update`
      (`self.K2_SetActorTransform` (`KismetMathLibrary.TLerp` (`self.Starting Transform`) (`self.Target Transform`) _progress)))
    (:`Finished`
      (bind _vfx_2 (`self.Play End Effects`))
      (`KismetSystemLibrary.Delay` 0.2)
      (`ActorComponent.Deactivate` _vfx)
      (`ActorComponent.Deactivate` _sfx)
      (`ActorComponent.Deactivate` _vfx_2)
      (`FXSystemComponent.ReleaseToPool` _vfx)
      (`FXSystemComponent.ReleaseToPool` _vfx_2)
      (`/Engine/EditorBlueprintResources/StandardMacros.IsValid` _sfx
        (:`Is Valid`
          (`ActorComponent.K2_DestroyComponent` _sfx))))))

(event `self.HandlePlayerOverlapEnd`
  (params (OtherActor :type "Actor Object Reference"))
  (`parent.HandlePlayerOverlapEnd` OtherActor)
  (bind _returnvalue (message `FormChangeActorInterface.GetFormChangeComponent` OtherActor))
  (`/Engine/EditorBlueprintResources/StandardMacros.IsValid` _returnvalue
    (:`Is Valid`
      (remove `PlayerFormChangeComponent.OnPlayerFormChange` _returnvalue (delegate `OnPlayerFormChange_Event`)))))

(event `OnPlayerFormChange_Event`
  (params (Payload :type "PlayerFormChangeEventPayload Structure (by ref)"))
  (`self.Handle Form Change` (stale `self.HandlePlayerOverlapBegin` OtherActor)))

(event `self.HandlePlayerOverlapBegin`
  (params (OtherActor :type "Actor Object Reference"))
  (`parent.HandlePlayerOverlapBegin` OtherActor)
  (bind _returnvalue (message `FormChangeActorInterface.GetFormChangeComponent` OtherActor))
  (`/Engine/EditorBlueprintResources/StandardMacros.IsValid` _returnvalue
    (:`Is Valid`
      (add `PlayerFormChangeComponent.OnPlayerFormChange` _returnvalue (delegate `OnPlayerFormChange_Event`)))))

(fn `GetHighlightMeshes`
  (returns (OutHighlightMeshes :type "Array of MeshComponent Object Reference"))
  (return (`|MakeArray` (`self.StaticMesh`) :!type "MeshComponent Object Reference")))

(fn `GetPreconditionIcon`
  (returns (ReturnValue :type "Texture2D Object Reference"))
  (return "/Game/Assets/UI/Portraits/T_Portrait_Barbarian.T_Portrait_Barbarian"))

(fn `Handle Form Change`
  (params (Player :type "Actor Object Reference"))
  (`self.HandlePlayerOverlapBegin` Player))

(fn `IsPreconditionMet`
  (params (Player :type "Actor Object Reference"))
  (returns (ReturnValue :type Boolean))
  (return (`GameplayTagAssetInterface.HasMatchingGameplayTag` (`ElectricCastleAbilitySystemLibrary.GetAbilitySystemComponent` Player) (struct :`TagName` "Player.Form.Barbarian"))))

(fn `OnInteract`
  (params (Player :type "Actor Object Reference"))
  (returns (ReturnValue :type Boolean))
  (`self.Knockdown` Player)
  (return true))

(fn `Play End Effects`
  (returns (VFX :type "NiagaraComponent Object Reference"))
  (`GameplayStatics.PlayWorldCameraShake` "/Game/FAB/Vefects/Zap_VFX/Shared/Cam/Cam_Shake_Slight.Cam_Shake_Slight_C" (`SceneComponent.K2_GetComponentLocation` (`self.Top`)) 0.0 (* (`KismetMathLibrary.Vector_Distance` (`SceneComponent.K2_GetComponentLocation` (`self.Effect Root`)) (`SceneComponent.K2_GetComponentLocation` (`self.Top`))) 1.5) 0.0)
  (`GameplayStatics.PlaySoundAtLocation` "/Game/Blueprints/LevelAssets/Knockdown/SFX/sfx_knockdown_impact.sfx_knockdown_impact" (`SceneComponent.K2_GetComponentLocation` (`self.Top`)) (struct) 1.0 1.0 0.0 "/Game/Assets/Sounds/Abilities/FireBolt/att_InWorld.att_InWorld" null self null)
  (bind _returnvalue (`NiagaraFunctionLibrary.SpawnSystemAttached` "/Game/Blueprints/LevelAssets/Knockdown/VFX/NS_Knockdown_ImpactEffect.NS_Knockdown_ImpactEffect" (`self.Top`) "None" (0.0 0.0 0.0) (struct) "KeepRelativeOffset" true true "ManualRelease"))
  (return _returnvalue))

(fn `Play Start Effects`
  (returns (SFX :type "AudioComponent Object Reference") (VFX :type "NiagaraComponent Object Reference"))
  (bind _returnvalue (`SceneComponent.K2_GetComponentLocation` (`self.Effect Root`)))
  (`GameplayStatics.PlayWorldCameraShake` "/Game/FAB/Vefects/Zap_VFX/Shared/Cam/Cam_Shake_Slight.Cam_Shake_Slight_C" _returnvalue 0.0 500.0)
  (bind _returnvalue_2 (`GameplayStatics.SpawnSoundAtLocation` "/Game/Blueprints/LevelAssets/Knockdown/SFX/sfx_knockdown_wood.sfx_knockdown_wood" _returnvalue (struct) 1.0 1.0 0.0 "/Game/Assets/Sounds/Abilities/FireBolt/att_InWorld.att_InWorld" null))
  (bind _returnvalue_3 (`NiagaraFunctionLibrary.SpawnSystemAttached` "/Game/Blueprints/LevelAssets/Knockdown/VFX/NS_Knockdown_DirtEffect.NS_Knockdown_DirtEffect" (`self.Effect Root`) "None" (0.0 0.0 0.0) (struct) "KeepRelativeOffset" true true "ManualRelease"))
  (return _returnvalue_2 _returnvalue_3))

(fn `UserConstructionScript`)