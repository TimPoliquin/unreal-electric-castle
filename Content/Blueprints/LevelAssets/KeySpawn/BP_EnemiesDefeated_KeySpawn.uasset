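; Actor that spawns a key when all enemies from a linked spawn volume are defeated.
; On BeginPlay it binds to the SpawnVolume's all-enemies-defeated event, if a volume is set.
; When that event fires, it spawns the configured key class at its own transform, adjusting for collision but always spawning.
; A HasSpawnedKey flag limits it to a single key.
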(event `self.ReceiveBeginPlay`
  (bind _spawn_volume (`self.Spawn Volume`)
    (:`then`
      (add `EnemySpawnVolume.OnAllEnemiesDefeated` _spawn_volume (delegate `OnAllEnemiesDefeated_Event`)))
    (:`else`)))

(event `OnAllEnemiesDefeated_Event`
  (if (not (`self.bHasSpawnedKey`))
    (`|SpawnActorFromClass` (`self.Key Class`) (`self.GetTransform`) "AdjustIfPossibleButAlwaysSpawn" "MultiplyWithRoot" self null)
    (set `self.bHasSpawnedKey` true)))

(fn `UserConstructionScript`)