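; Possessable statue puzzle piece that the Magic Hand can rotate in 90-degree snaps to drive linked trigger actors.
; A snap-mode RotationTetherHandler fires on each snap, playing a sound and line-tracing along the statue's forward vector.
; Each actor in Triggers then receives a bool that is true when it is absent from the trace result.
; Possession blends to the statue's detached camera, blocks offensive abilities and enables vision FX and highlight until release.
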(event `self.ReceiveBeginPlay`
  (bind _returnvalue (`|GenericCreateObject` "/Script/ElectricCastle.RotationTetherHandler" "Snap" 1.0 90.0 90.0))
  (set `self.Tether Update Handler` _returnvalue)
  (`self.Setup Rotation Snap Listener`)
  (`CameraMovementModifier.SetCameraComponent` (`self.Camera Input Modifier`) (`self.Possession Camera`)))

(event `Setup Rotation Snap Listener`
  (add `RotationTetherHandler.OnRotationSnap` (`self.Tether Update Handler`) (delegate `OnRotationSnap_Event`)))

(event `OnRotationSnap_Event`
  (params (Payload :type "RotationTetherHandlerEventPayload Structure (by ref)"))
  (`GameplayStatics.PlaySoundAtLocation` (`self.Rotation Sound`) (`self.K2_GetActorLocation`) (struct) 2.0 1.0 0.0 "/Game/Assets/Sounds/Abilities/FireBolt/att_InWorld.att_InWorld" null self null)
  (bind _out_hit_actors (`self.Trace for Targets`))
  (`self.Trigger Actors` _out_hit_actors))

(event `self.OnPossessionStarted`
  (params (Payload :type "MagicHandPossessEventPayload Structure (by ref)"))
  (bind _returnvalue (`PlayerFunctionLibrary.GetPlayerController` Payload_PossessorActor))
  (`/Engine/EditorBlueprintResources/StandardMacros.IsValid` _returnvalue
    (:`Is Valid`
      (`PlayerController.SetViewTargetWithBlend` _returnvalue Payload_PossessedActor 1.5 "VTBlend_EaseInOut" 1.0 false)
      (`SceneComponent.K2_DetachFromComponent` (`self.Possession Camera`) "KeepWorld" "KeepWorld" "KeepRelative" true)
      (bind _returnvalue_2 (`ElectricCastleAbilitySystemLibrary.ApplyInfiniteEffectByTags` Payload_PossessorActor (struct :`GameplayTags` (struct :`(TagName` "Player.Block.Ability.Offensive") :`(TagName` "Player.Block.Interaction") :`(TagName` "Player.Block.Rotation") :`(TagName` "Player.Block.ChangeForm") :`(TagName` "Player.Block.LockOn") :`(TagName` "Player.Block.Look")))))
      (set `self.Player Block Look Effect Handle` _returnvalue_2)
      (`ActorComponent.Activate` (`self.VisionFX`) false)
      (`HighlightComponent.Highlight` (`self.Highlight`)))))

(event `self.OnPossessionEnded`
  (params (Payload :type "MagicHandPossessEventPayload Structure (by ref)"))
  (bind _returnvalue (`PlayerFunctionLibrary.GetPlayerController` Payload_PossessorActor))
  (`/Engine/EditorBlueprintResources/StandardMacros.IsValid` _returnvalue
    (:`Is Valid`
      (`PlayerController.SetViewTargetWithBlend` _returnvalue Payload_PossessorActor 1.0 "VTBlend_EaseInOut" 1.5 false)
      (`SceneComponent.K2_AttachToComponent` (`self.Possession Camera`) (`self.RootComponent`) "None" "KeepWorld" "KeepWorld" "KeepWorld" true)
      (`ActorComponent.Deactivate` (`self.VisionFX`))
      (`HighlightComponent.Unhighlight` (`self.Highlight`))
      (`KismetSystemLibrary.Delay` 1.0)
      (`ElectricCastleAbilitySystemLibrary.RemoveGameplayEffect` Payload_PossessorActor (`self.Player Block Look Effect Handle`) false true))))

(fn `CanBePossessedByMagicHand`
  (returns (ReturnValue :type Boolean))
  (return true))

(fn `GetCameraMovementModifier`
  (returns (ReturnValue :type "CameraMovementModifier Object Reference"))
  (return (`self.Camera Input Modifier`)))

(fn `GetHighlightComponent`
  (returns (ReturnValue :type "HighlightComponent Object Reference"))
  (return (`self.Highlight`)))

(fn `GetHighlightMeshes`
  (returns (OutHighlightMeshes :type "Array of MeshComponent Object Reference"))
  (return (`|MakeArray` (`self.Statue Mesh`) :!type "MeshComponent Object Reference")))

(fn `GetTetherUpdateHandler`
  (returns (ReturnValue :type "TetherUpdateHandler Object Reference"))
  (return (`self.Tether Update Handler`)))

(fn `Hit Results to Actors`
  (params (HitResults :type "Array of HitResult Structure"))
  (returns (`Out Hit Actors` :type "Set of Actor Object Reference"))
  (locals (`Hit Actors` :type "Set of Actor Object Reference"))
  (for _array_element HitResults
    (`BlueprintSetLibrary.Set_Add` (`local.Hit Actors`) (`.HitActor` (`GameplayStatics.BreakHitResult` _array_element)))
    (return (`local.Hit Actors`))))

(fn `Trace for Targets`
  (returns (`Out Hit Actors` :type "Set of Actor Object Reference"))
  (bind _returnvalue (`SceneComponent.K2_GetComponentLocation` (`self.Trace Origin`)))
  (bind _outhits (`KismetSystemLibrary.LineTraceMultiByProfile` _returnvalue (+ _returnvalue (* (`self.GetActorForwardVector`) (`self.Line Trace Range`))) "Trigger"))
  (return (`self.Hit Results to Actors` _outhits)))

(fn `Trigger Actors`
  (params (TargetSet :type "Set of Actor Object Reference (by ref)"))
  (for _array_element (`self.Triggers`)
    (message `TriggerableInterface.OnTrigger` _array_element (not (`BlueprintSetLibrary.Set_Contains` TargetSet _array_element)))))

(fn `UserConstructionScript`)