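; Turret level actor that fires projectiles from its spawn point on a looping timer while active.
; Once game data is loaded, it starts the fire timer and builds damage effect params from DamageConfig using its ability system and GE_BasicDamage.
; Each projectile receives those params and a configured speed at spawn.
; Triggers toggle Active, pausing or unpausing the timer, and IsTriggered reports that state.
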(event `self.ReceiveBeginPlay`
  (bind _returnvalue (subsystem `ElectricCastleGameDataSubsystem`))
  (if (`ElectricCastleGameDataSubsystem.IsGameDataLoaded` _returnvalue)
    (`self.OnGameDataLoaded_Event`)
    (else
      (add `ElectricCastleGameDataSubsystem.OnGameDataLoaded` _returnvalue (delegate `OnGameDataLoaded_Event`)))))

(event `OnGameDataLoaded_Event`
  (bind _returnvalue (`KismetSystemLibrary.K2_SetTimerDelegate` (delegate `Fire`) (`self.Fire Rate`) true))
  (set `self.Fire Timer Handle` _returnvalue)
  (bind _newparam (`self.Make Damage Effect Params`))
  (set `self.Damage Params` _newparam))

(event `Fire`
  (if (`self.Active`)
    (`self.Spawn Projectile`)
    (else
      (`KismetSystemLibrary.K2_PauseTimerHandle` (`self.Fire Timer Handle`)))))

(event `TriggerInterface.OnTrigger`
  (params (InActivate :type Boolean))
  (`self.Set Active` InActivate))

(event `Set Active`
  (params (`Is Active` :type Boolean))
  (bind _output_get (set `self.Active` `Is Active`))
  (if _output_get
    (`KismetSystemLibrary.K2_UnPauseTimerHandle` (`self.Fire Timer Handle`))
    (else
      (`KismetSystemLibrary.K2_PauseTimerHandle` (`self.Fire Timer Handle`)))))

(fn `IsTriggered`
  (returns (ReturnValue :type Boolean))
  (return (`self.Active`)))

(fn `Make Damage Effect Params`
  (returns (NewParam :type "DamageEffectParams Structure"))
  (bind (_damage_config_damagetypetag _damage_config_damagemagnitude _damage_config_debuffchance _damage_config_debuffdamage _damage_config_debufffrequency _damage_config_debuffduration _damage_config_deathimpulsemagnitude _damage_config_knockbackforcemagnitude _damage_config_knockbackchance _damage_config_bisradialdamage _damage_config_radialdamageinnerradius _damage_config_radialdamageouterradius) (break `ElectricCastleDamageConfig` (`self.Damage Config`)))
  (return (make `DamageEffectParams` self "/Game/Blueprints/AbilitySystem/GameplayEffects/GE_BasicDamage.GE_BasicDamage_C" (`self.AbilitySystem`) null (`AbilitySystemBlueprintLibrary.Conv_ScalableFloatToFloat` _damage_config_damagemagnitude 1.0) 1.0 _damage_config_damagetypetag _damage_config_debuffchance _damage_config_debuffdamage _damage_config_debuffduration _damage_config_debufffrequency _damage_config_deathimpulsemagnitude (0.0 0.0 0.0) _damage_config_knockbackchance _damage_config_knockbackforcemagnitude (0.0 0.0 0.0) _damage_config_bisradialdamage _damage_config_radialdamageinnerradius _damage_config_radialdamageouterradius)))

(fn `Spawn Projectile`
  (`|SpawnActorFromClass` (`self.Projectile`) (`SceneComponent.K2_GetComponentToWorld` (`self.Projectile Spawn Point`)) "AlwaysSpawn" "MultiplyWithRoot" self (`self.Speed`) (`self.Damage Params`) null (struct) null))

(fn `UserConstructionScript`)