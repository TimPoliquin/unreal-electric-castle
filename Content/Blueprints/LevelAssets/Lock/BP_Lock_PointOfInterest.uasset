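; BP_Lock_PointOfInterest is a lock point of interest that shows a key mesh once unlocked and marks itself with an important POI icon while locked.
; On BeginPlay it runs post-load logic after the parent's, setting key mesh visibility from the Unlocked state.
; When locked, it also sets the Important icon on its POI widget.
; PlayUnlockEffect reveals the key mesh and its children.
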(event `self.ReceiveBeginPlay`
  (`SaveableInterface.PostLoad`))

(event `SaveableInterface.PostLoad`
  (`parent.PostLoad`)
  (if (`self.bUnlocked`)
    (`SceneComponent.SetVisibility` (`self.Unlocked Key Mesh Component`) true false)
    (else
      (`SceneComponent.SetVisibility` (`self.Unlocked Key Mesh Component`) false true)
      (`self.Initialize POI Icon`))))

(event `self.PlayUnlockEffect`
  (params (Player :type "Actor Object Reference"))
  (`SceneComponent.SetVisibility` (`self.Unlocked Key Mesh Component`) true true))

(fn `Initialize POI Icon`
  (bind _aswbp_poi (cast `/Game/Blueprints/UI/POI/WBP_POI` (`WidgetComponent.GetWidget` (`self.POIWidget`))))
  (set `/Game/Blueprints/UI/POI/WBP_POI.POI_Icon` "/Game/Assets/UI/Icons/important_256.important_256" _aswbp_poi))

(fn `UserConstructionScript`)