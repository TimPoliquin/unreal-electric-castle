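; Test level manager actor that shows or hides a Target actor based on the state of a linked Button switch.
; On BeginPlay it binds to the Button's activated and deactivated delegates and applies the switch's current state.
; Activation makes the Target visible and deactivation hides it, with validity checks on both references.
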(event `self.ReceiveBeginPlay`
  (bind _button (`self.Button`)
    (:`then`
      (add `ButtonSwitchActor.OnActivatedDelegate` _button (delegate `OnActivatedDelegate_Event`))
      (add `ButtonSwitchActor.OnDeactivatedDelegate` (`self.Button`) (delegate `OnDeactivatedDelegate_Event`))
      (if (`SwitchInterface.IsSwitchActive` (`self.Button`))
        (`self.Handle Button Activate`)
        (else
          (`self.Handle Button Deactivate`))))
    (:`else`)))

(event `OnActivatedDelegate_Event`
  (params (Payload :type "OnSwitchStatusChangedPayload Structure (by ref)"))
  (`self.Handle Button Activate`))

(event `OnDeactivatedDelegate_Event`
  (params (Payload :type "OnSwitchStatusChangedPayload Structure (by ref)"))
  (`self.Handle Button Deactivate`))

(event `Handle Button Activate`
  (bind _target (`self.Target`)
    (:`then`
      (`StateShiftBlueprintFunctionLibrary.SetActorVisibility` _target true))
    (:`else`)))

(event `Handle Button Deactivate`
  (bind _target (`self.Target`)
    (:`then`
      (`StateShiftBlueprintFunctionLibrary.SetActorVisibility` _target))
    (:`else`)))

(fn `UserConstructionScript`)