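; BP_Puzzle_ButtonManager is a puzzle room controller that traps the player until a linked button is activated.
; A player overlapping the entry collider while unsolved closes and locks the Door and triggers the lock-activation list.
; The button's activation delegate marks the puzzle solved, disables the collider, unlocks and opens the Door, and sends on/off trigger messages to the unlock lists.
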(event `self.ReceiveBeginPlay`
  (bind _button (`self.Button`)
    (:`then`
      (add `ButtonSwitchActor.OnActivatedDelegate` _button (delegate `OnActivatedDelegate_Event`)))
    (:`else`)))

(event `OnActivatedDelegate_Event`
  (params (Payload :type "OnSwitchStatusChangedPayload Structure (by ref)"))
  (`self.Handle Button Activate`))

(event `Handle Button Activate`
  (`self.Solve`))

(event `self.Room Enter Collider.OnComponentBeginOverlap`
  (params (OverlappedComponent :type "PrimitiveComponent Object Reference") (OtherActor :type "Actor Object Reference") (OtherComp :type "PrimitiveComponent Object Reference") (OtherBodyIndex :type Integer) (bFromSweep :type Boolean) (SweepResult :type "HitResult Structure (by ref)"))
  (if (and (`KismetSystemLibrary.DoesImplementInterface` OtherActor "/Script/ElectricCastle.PlayerInterface") (not (`self.Solved`)))
    (`self.Lock Room`)))

(event `Solve`
  (set `self.Solved` true)
  (set `self.IsLocked` false)
  (`ActorComponent.Deactivate` (`self.Room Enter Collider`))
  (`/Game/Blueprints/LevelAssets/LevelPrototyping/Interactable/Door/BP_DoorFrame.Unlock` (`self.Door`))
  (`/Game/Blueprints/LevelAssets/LevelPrototyping/Interactable/Door/BP_DoorFrame.Open Door` (`self.Door`))
  (for _array_element (`self.ToActivateOnUnlock`)
    (message `/Game/Blueprints/LevelAssets/Button/BI_Triggerable.OnTrigger` _array_element true))
  (for _array_element_2 (`self.ToDeactivateOnUnlock`)
    (message `/Game/Blueprints/LevelAssets/Button/BI_Triggerable.OnTrigger` _array_element_2 false)))

(event `Lock Room`
  (bind _door (`self.Door`))
  (if (not (`self.IsLocked`))
    (set `self.IsLocked` true)
    (`/Game/Blueprints/LevelAssets/LevelPrototyping/Interactable/Door/BP_DoorFrame.Close Door` _door)
    (`/Game/Blueprints/LevelAssets/LevelPrototyping/Interactable/Door/BP_DoorFrame.Lock` _door)
    (for _array_element (`self.ToActivateOnLock`)
      (message `/Game/Blueprints/LevelAssets/Button/BI_Triggerable.OnTrigger` _array_element true))))

(fn `UserConstructionScript`)