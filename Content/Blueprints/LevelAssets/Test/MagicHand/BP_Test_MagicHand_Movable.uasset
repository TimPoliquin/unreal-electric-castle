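; Test movable cube actor that the Magic Hand can always possess.
; On BeginPlay it creates a debug-enabled PhysicsMovementTetherHandler, exposed through a getter, and a dynamic transparent material for the cube, unless a handler already exists.
; Possession deactivates its BasicGravity component and makes the cube semi-transparent; ending possession restores both gravity and full opacity.
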(event `self.ReceiveBeginPlay`
  (`self.TetherUpdateHandler`
    (:`then`)
    (:`else`
      (bind _returnvalue (`|GenericCreateObject` "/Script/ElectricCastle.PhysicsMovementTetherHandler" 150.0 150.0 25.0 true))
      (set `self.TetherUpdateHandler` _returnvalue)
      (bind _returnvalue_2 (`PrimitiveComponent.CreateDynamicMaterialInstance` (`self.Cube`) 0 "/Game/Blueprints/LevelAssets/Test/Material/MI_BasicTransparent.MI_BasicTransparent" "None"))
      (set `self.Dynamic Material` _returnvalue_2))))

(event `self.OnPossessionStarted`
  (params (MagicHandComponent :type "MagicHandComponent Object Reference"))
  (`ActorComponent.Deactivate` (`self.BasicGravity`))
  (`MaterialInstanceDynamic.SetScalarParameterValue` (`self.Dynamic Material`) "Opacity" 0.5))

(event `self.OnPossessionEnded`
  (`ActorComponent.Activate` (`self.BasicGravity`) false)
  (`MaterialInstanceDynamic.SetScalarParameterValue` (`self.Dynamic Material`) "Opacity" 1.0))

(fn `CanBePossessedByMagicHand`
  (returns (ReturnValue :type Boolean))
  (return true))

(fn `GetTetherUpdateHandler`
  (returns (ReturnValue :type "TetherUpdateHandler Object Reference"))
  (return (`self.TetherUpdateHandler`)))

(fn `UserConstructionScript`)