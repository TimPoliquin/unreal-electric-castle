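; Test actor that the Magic Hand can possess and rotate, serving as a key for triggers and locks.
; On BeginPlay it creates a snapping RotationTetherHandler for quarter turns and a transparent dynamic material.
; Possession turns off gravity and fades the cube to half opacity until released.
; FacingTargetCollision overlaps with listed TargetTriggers unlock or trigger them through interfaces, reversing both once overlap fully ends.
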(event `self.ReceiveBeginPlay`
  (`self.TetherUpdateHandler`
    (:`then`)
    (:`else`
      (bind _returnvalue (`|GenericCreateObject` "/Script/ElectricCastle.RotationTetherHandler" "Snap" 1.0 90.0 90.0))
      (set `self.TetherUpdateHandler` _returnvalue)
      (bind _returnvalue_2 (`PrimitiveComponent.CreateDynamicMaterialInstance` (`self.Cube`) 0 "/Game/Blueprints/LevelAssets/Test/Material/MI_BasicTransparent.MI_BasicTransparent" "None"))
      (set `self.Dynamic Material` _returnvalue_2))))

(event `self.OnPossessionStarted`
  (params (MagicHandComponent :type "MagicHandComponent Object Reference"))
  (`ActorComponent.Deactivate` (`self.BasicGravity`))
  (`MaterialInstanceDynamic.SetScalarParameterValue` (`self.Dynamic Material`) "Opacity" 0.5))

(event `self.OnPossessionEnded`
  (`ActorComponent.Activate` (`self.BasicGravity`) false)
  (`MaterialInstanceDynamic.SetScalarParameterValue` (`self.Dynamic Material`) "Opacity" 1.0))

(event `self.Facing Target Collision.OnComponentBeginOverlap`
  (params (OverlappedComponent :type "PrimitiveComponent Object Reference") (OtherActor :type "Actor Object Reference") (OtherComp :type "PrimitiveComponent Object Reference") (OtherBodyIndex :type Integer) (bFromSweep :type Boolean) (SweepResult :type "HitResult Structure (by ref)"))
  (`KismetSystemLibrary.PrintString` (`KismetSystemLibrary.GetObjectName` OtherActor))
  (if (`KismetArrayLibrary.Array_Contains` (`self.Target Triggers`) OtherActor)
    (`|ExecutionSequence`
      (:`then_0`
        (if (`KismetSystemLibrary.DoesImplementInterface` OtherActor "/Script/ElectricCastle.LockInterface")
          (message `LockInterface.Unlock` OtherActor)))
      (:`then_1`
        (if (`KismetSystemLibrary.DoesImplementInterface` OtherActor "/Script/ElectricCastle.TriggerableInterface")
          (message `TriggerableInterface.OnTrigger` OtherActor true))))))

(event `self.Facing Target Collision.OnComponentEndOverlap`
  (params (OverlappedComponent :type "PrimitiveComponent Object Reference") (OtherActor :type "Actor Object Reference") (OtherComp :type "PrimitiveComponent Object Reference") (OtherBodyIndex :type Integer))
  (if (and (`KismetArrayLibrary.Array_Contains` (`self.Target Triggers`) OtherActor) (not (`PrimitiveComponent.IsOverlappingActor` (`self.Facing Target Collision`) OtherActor)))
    (`|ExecutionSequence`
      (:`then_0`
        (if (`KismetSystemLibrary.DoesImplementInterface` OtherActor "/Script/ElectricCastle.TriggerableInterface")
          (message `TriggerableInterface.OnTrigger` OtherActor false)))
      (:`then_1`
        (if (`KismetSystemLibrary.DoesImplementInterface` OtherActor "/Script/ElectricCastle.LockInterface")
          (message `LockInterface.Lock` OtherActor))))))

(fn `CanBePossessedByMagicHand`
  (returns (ReturnValue :type Boolean))
  (return true))

(fn `GetTetherUpdateHandler`
  (returns (ReturnValue :type "TetherUpdateHandler Object Reference"))
  (return (`self.TetherUpdateHandler`)))

(fn `UserConstructionScript`)