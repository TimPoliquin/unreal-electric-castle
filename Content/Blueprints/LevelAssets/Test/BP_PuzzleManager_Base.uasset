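; Base puzzle room manager that locks the player in on entry and releases them when the puzzle is solved.
; A collider overlap from a PlayerInterface actor calls LockRoom, which closes and locks the Door unless already locked or solved.
; Solve disables the collider, opens the Door and plays a success sound.
; Both transitions send activate or deactivate messages to configurable trigger lists via ExecuteTriggers.
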(event `self.Room Enter Collider.OnComponentBeginOverlap`
  (params (OverlappedComponent :type "PrimitiveComponent Object Reference") (OtherActor :type "Actor Object Reference") (OtherComp :type "PrimitiveComponent Object Reference") (OtherBodyIndex :type Integer) (bFromSweep :type Boolean) (SweepResult :type "HitResult Structure (by ref)"))
  (if (and (`KismetSystemLibrary.DoesImplementInterface` OtherActor "/Script/ElectricCastle.PlayerInterface") (not (`self.Solved`)))
    (`self.Lock Room`)))

(event `Solve`
  (set `self.Solved` true)
  (set `self.IsLocked` false)
  (`ActorComponent.Deactivate` (`self.Room Enter Collider`))
  (`/Game/Blueprints/LevelAssets/LevelPrototyping/Interactable/Door/BP_DoorFrame.Unlock` (`self.Door`))
  (`/Game/Blueprints/LevelAssets/LevelPrototyping/Interactable/Door/BP_DoorFrame.Open Door` (`self.Door`))
  (`GameplayStatics.PlaySound2D` "/Game/Assets/Sounds/Fishing/SFX_Success.SFX_Success" 1.0 1.0 0.0 null null)
  (`self.Execute Triggers` (`self.ToActivateOnUnlock`) true)
  (`self.Execute Triggers` (`self.ToDeactivateOnUnlock`)))

(event `Lock Room`
  (bind _door (`self.Door`))
  (if (not (`self.IsLocked`))
    (set `self.IsLocked` true)
    (`/Game/Blueprints/LevelAssets/LevelPrototyping/Interactable/Door/BP_DoorFrame.Close Door` _door)
    (`/Game/Blueprints/LevelAssets/LevelPrototyping/Interactable/Door/BP_DoorFrame.Lock` _door)
    (`self.Execute Triggers` (`self.ToActivateOnLock`) true)
    (`self.Execute Triggers` (`self.ToDeactivateOnLock`))))

(fn `Execute Triggers`
  (params (Triggers :type "Array of Actor Object Reference") (Activate :type Boolean))
  (for _array_element Triggers
    (message `/Game/Blueprints/LevelAssets/Button/BI_Triggerable.OnTrigger` _array_element (`local.Activate`))))

(fn `UserConstructionScript`)