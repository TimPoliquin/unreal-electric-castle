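; Legacy hover cart variant that follows a track and, when AllowMagicHandPossession is set, can be possessed by the magic hand.
; It constructs a TrackTetherHandler on BeginPlay if possession is allowed, and again whenever a track is set, regardless of that flag.
; Getters expose the track-following component and the mesh as hand attach point.
; GetUpdateTetherHandler returns nothing, so the stored handler is never read here.
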(event `self.ReceiveBeginPlay`
  (`parent.ReceiveBeginPlay`)
  (if (`self.Allow Magic Hand Possession`)
    (`self.Create Track Tether Update Handler`)))

(event `self.Set Track`
  (params (InTrack :type "SplineComponent Object Reference"))
  (`parent.Set Track` InTrack)
  (`self.Create Track Tether Update Handler`))

(fn `CanBePossessedByMagicHand`
  (returns (ReturnValue :type Boolean))
  (return (`self.Allow Magic Hand Possession`)))

(fn `Create Track Tether Update Handler`
  (bind _returnvalue (`|GenericCreateObject` "/Script/ElectricCastle.TrackTetherHandler" null))
  (set `self.Tether Update Handler` _returnvalue))

(fn `GetMagicHandAttachComponent`
  (returns (AttachBoneName :type Name) (ReturnValue :type "SceneComponent Object Reference"))
  (return "None" (`self.Mesh Component`)))

(fn `GetTrackFollowingComponent`
  (returns (ReturnValue :type "TrackFollowingComponent Object Reference"))
  (return (`self.TrackFollowing`)))

(fn `GetUpdateTetherHandler`
  (returns (ReturnValue :type "UpdateTetherHandler Object Reference"))
  (return null))

(fn `UserConstructionScript`
  (`parent.UserConstructionScript`))