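; BP_HoverCart is a test-level hover cart that moves along an assigned track through its TrackFollowing component.
; Player interaction toggles movement, with stopping gated by AllowManualDeactivation, while triggers can only start it.
; ReturnToStart and ReturntoEnd set reverse or forward direction and activate the component.
; An overlap volume applies the GE_InteractAvailable gameplay effect to the player on entry and removes it by stored handle on exit.
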(event `Set Track`
  (params (InTrack :type "SplineComponent Object Reference"))
  (`TrackFollowingComponent.SetTrack` (`self.TrackFollowing`) InTrack))

(event `Toggle Active`
  (if (not (`ActorComponent.IsActive` (`self.TrackFollowing`)))
    (`ActorComponent.Activate` (`self.TrackFollowing`) false)
    (elif (`self.Allow Manual Deactivation`)
      (`ActorComponent.Deactivate` (`self.TrackFollowing`)))))

(event `self.Interaction Collision.OnComponentBeginOverlap`
  (params (OverlappedComponent :type "PrimitiveComponent Object Reference") (OtherActor :type "Actor Object Reference") (OtherComp :type "PrimitiveComponent Object Reference") (OtherBodyIndex :type Integer) (bFromSweep :type Boolean) (SweepResult :type "HitResult Structure (by ref)"))
  (bind _asbp_player_character (cast `/Game/Blueprints/Player/BP_PlayerCharacter` OtherActor))
  (bind _returnvalue (`ElectricCastleAbilitySystemLibrary.ApplyBasicGameplayEffect` _asbp_player_character "/Game/Blueprints/AbilitySystem/GameplayEffects/GE_InteractAvailable.GE_InteractAvailable_C"))
  (set `self.Interaction Effect Handle` _returnvalue))

(event `self.Interaction Collision.OnComponentEndOverlap`
  (params (OverlappedComponent :type "PrimitiveComponent Object Reference") (OtherActor :type "Actor Object Reference") (OtherComp :type "PrimitiveComponent Object Reference") (OtherBodyIndex :type Integer))
  (bind _asbp_player_character (cast `/Game/Blueprints/Player/BP_PlayerCharacter` OtherActor))
  (`ElectricCastleAbilitySystemLibrary.RemoveGameplayEffect` _asbp_player_character (`self.Interaction Effect Handle`) false true))

(event `self.OnTrigger`
  (params (InActivate :type Boolean))
  (if InActivate
    (`ActorComponent.Activate` (`self.TrackFollowing`) false)))

(event `Return To Start`
  (bind _trackfollowing (`self.TrackFollowing`))
  (`TrackFollowingComponent.SetDirection` _trackfollowing "Reverse")
  (`ActorComponent.Activate` _trackfollowing false))

(event `Return to End`
  (bind _trackfollowing (`self.TrackFollowing`))
  (`TrackFollowingComponent.SetDirection` _trackfollowing "Forward")
  (`ActorComponent.Activate` _trackfollowing false))

(fn `GetTrackFollowingComponent`
  (returns (ReturnValue :type "TrackFollowingComponent Object Reference"))
  (return (`self.TrackFollowing`)))

(fn `OnInteract`
  (params (Player :type "Actor Object Reference"))
  (returns (ReturnValue :type Boolean))
  (`self.Toggle Active`)
  (return true))

(fn `UserConstructionScript`)