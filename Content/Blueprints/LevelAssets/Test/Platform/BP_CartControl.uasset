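; BP_CartControl is an interactable control, likely for a cart, that fires trigger actions when a player uses it.
; Its Box applies the GE_InteractAvailable gameplay effect to overlapping PlayerInterface actors and removes it on exit using the stored handle.
; OnInteract calls ExecuteTriggerActions on Trigger and reports success.
; The end-overlap interface check names no interface, unlike the begin-overlap check.
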(event `self.Box.OnComponentBeginOverlap`
  (params (OverlappedComponent :type "PrimitiveComponent Object Reference") (OtherActor :type "Actor Object Reference") (OtherComp :type "PrimitiveComponent Object Reference") (OtherBodyIndex :type Integer) (bFromSweep :type Boolean) (SweepResult :type "HitResult Structure (by ref)"))
  (if (`KismetSystemLibrary.DoesImplementInterface` OtherActor "/Script/ElectricCastle.PlayerInterface")
    (bind _returnvalue (`ElectricCastleAbilitySystemLibrary.ApplyBasicGameplayEffect` OtherActor "/Game/Blueprints/AbilitySystem/GameplayEffects/GE_InteractAvailable.GE_InteractAvailable_C"))
    (set `self.Interaction Effect Handle` _returnvalue)))

(event `self.Box.OnComponentEndOverlap`
  (params (OverlappedComponent :type "PrimitiveComponent Object Reference") (OtherActor :type "Actor Object Reference") (OtherComp :type "PrimitiveComponent Object Reference") (OtherBodyIndex :type Integer))
  (if (`KismetSystemLibrary.DoesImplementInterface` OtherActor)
    (`ElectricCastleAbilitySystemLibrary.RemoveGameplayEffect` OtherActor (`self.Interaction Effect Handle`) false true)))

(fn `OnInteract`
  (params (Player :type "Actor Object Reference"))
  (returns (ReturnValue :type Boolean))
  (`TriggerComponent.ExecuteTriggerActions` (`self.Trigger`))
  (return true))

(fn `UserConstructionScript`)