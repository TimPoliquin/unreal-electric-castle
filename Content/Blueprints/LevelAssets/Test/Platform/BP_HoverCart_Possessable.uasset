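; BP_HoverCart_Possessable is a hover cart in the test platform assets that the magic hand can possess.
; On BeginPlay it constructs a TrackTetherHandler from its TrackFollowing track spline, passing along the debug setting, and stores it.
; It always allows possession and exposes that handler through GetTetherUpdateHandler, while construction defers to the parent class.
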(event `self.ReceiveBeginPlay`
  (`parent.ReceiveBeginPlay`)
  (bind _returnvalue (`|GenericCreateObject` "/Script/ElectricCastle.TrackTetherHandler" (`TrackFollowingComponent.Track` (`self.TrackFollowing`)) 5.0 (`self.bDebug`)))
  (set `self.Tether Update Handler` _returnvalue))

(fn `CanBePossessedByMagicHand`
  (returns (ReturnValue :type Boolean))
  (return true))

(fn `GetTetherUpdateHandler`
  (returns (ReturnValue :type "TetherUpdateHandler Object Reference"))
  (return (`self.Tether Update Handler`)))

(fn `UserConstructionScript`
  (`parent.UserConstructionScript`))