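; Test actor that the Magic Hand can possess, with a Cube mesh and a BasicGravity component.
; It always allows possession and supplies its Highlight component, the Cube as highlight mesh, and the Cube as attach component with no bone.
; BasicGravity deactivates while the hand possesses the actor and reactivates on unpossess.
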(event `MagicHandPossessableInterface.OnMagicHandPossess`
  (`ActorComponent.Deactivate` (`self.BasicGravity`)))

(event `MagicHandPossessableInterface.OnMagicHandUnpossess`
  (`ActorComponent.Activate` (`self.BasicGravity`) false))

(fn `CanBePossessedByMagicHand`
  (returns (ReturnValue :type Boolean))
  (return true))

(fn `GetHighlightComponent`
  (returns (ReturnValue :type "HighlightComponent Object Reference"))
  (return (`self.Highlight`)))

(fn `GetHighlightMeshes`
  (returns (OutHighlightMeshes :type "Array of MeshComponent Object Reference"))
  (return (`|MakeArray` (`self.Cube`) :!type "MeshComponent Object Reference")))

(fn `GetMagicHandAttachComponent`
  (returns (AttachBoneName :type Name) (ReturnValue :type "SceneComponent Object Reference"))
  (return "None" (`self.Cube`)))

(fn `UserConstructionScript`)