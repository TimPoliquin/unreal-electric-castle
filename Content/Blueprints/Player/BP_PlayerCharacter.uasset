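; Player character Blueprint that adds aim camera zoom, a status effect bar and MetaHuman setup on top of its parent class.
; Aim start and end play timelines that lerp the spring arm from its current length toward the aim length or the default cached at BeginPlay.
; BeginPlay binds the status effect widget to the StatusEffectManagerComponent.
; GetMovementMode selects one of three modes from weapon-equipped and aiming state.
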(event `self.ReceiveBeginPlay`
  (`parent.ReceiveBeginPlay`)
  (`self.Bind Status Effect Widget Dependencies`)
  (set `self.Default Spring Arm Length` (`SpringArmComponent.TargetArmLength` (`self.SpringArmComponent`))))

(event `self.AimStart`
  (`parent.AimStart`)
  (bind (_direction _alpha) (`Timeline|Aim Start` :!via `PlayFromStart`)
    (:`Update`
      (`self.Update Spring Arm Length` (`self.Aim Spring Arm Length`) _alpha))))

(event `self.AimEnd`
  (`parent.AimEnd`)
  (bind (_direction _alpha) (`Timeline|Timeline` :!via `PlayFromStart`)
    (:`Update`
      (`self.Update Spring Arm Length` (`self.Default Spring Arm Length`) _alpha))))

(fn `Bind Status Effect Widget Dependencies`
  (bind _asstatus_effect_bar_widget (cast `StatusEffectBarWidget` (`WidgetComponent.GetWidget` (`self.Status Effects Widget`))))
  (`StatusEffectBarWidget.BindDependencies` _asstatus_effect_bar_widget (`self.StatusEffectManagerComponent`)))

(fn `GetMovementMode`
  (returns (`Movement Mode` :type "/Game/MetaHumans/Common/CharacterMovementMode Enum"))
  (locals (`Out Movement Mode` :type "/Game/MetaHumans/Common/CharacterMovementMode Enum" :default "NewEnumerator0"))
  (if (`PlayerFunctionLibrary.HasWeaponEquipped` null)
    (if (`PlayerFunctionLibrary.IsPlayerAiming` null)
      (set `local.Out Movement Mode` "NewEnumerator2")
      (else
        (set `local.Out Movement Mode` "NewEnumerator1")))
    (else
      (set `local.Out Movement Mode` "NewEnumerator0")))
  (return (`local.Out Movement Mode`)))

(fn `Update Spring Arm Length`
  (params (`Target Arm Length` :type "Float (double-precision)") (Alpha :type "Float (double-precision)"))
  (set `SpringArmComponent.TargetArmLength` (`KismetMathLibrary.Lerp` (`SpringArmComponent.TargetArmLength` (`self.SpringArmComponent`)) `Target Arm Length` Alpha) (`self.SpringArmComponent`)))

(fn `UserConstructionScript`
  (`self.Construction_SetupMetaHuman`))