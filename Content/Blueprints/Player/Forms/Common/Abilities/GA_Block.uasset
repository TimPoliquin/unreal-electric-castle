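; Player block ability that guards while input is held, with a level-scaled, delayed parry window at the start.
; It drives the avatar's block controller and reacts to block and parry gameplay events with sound and sparks; blocked hits also play a montage.
; A parry turns toward the attacker, applies a block-damage effect and plays a montage whose Land event staggers them.
; Releasing input ends the ability unless parrying; ending clears parry effects.
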(event `self.K2_ActivateAbility`
  (bind _returnvalue (`self.K2_CommitAbility`))
  (if _returnvalue
    (`self.Clear Parry Effect Handles`)
    (bind _returnvalue_2 (message `BlockingActorInterface.GetBlockController` (`self.GetAvatarActorFromActorInfo`)))
    (`/Engine/EditorBlueprintResources/StandardMacros.IsValid` _returnvalue_2
      (:`Is Valid`
        (`BlockController.StartBlocking` _returnvalue_2)
        (`self.Manage Parry Window`)
        (`self.Manage Block Hit`)
        (`AbilityTask_WaitInputRelease.WaitInputRelease` false
          (:`then`
            (`GameplayStatics.PlaySoundAtLocation` "/Game/Assets/Sounds/Abilities/Guard/SFX_Guard.SFX_Guard" (`Actor.K2_GetActorLocation` (`self.GetAvatarActorFromActorInfo`)) (struct) 1.0 1.0 0.0 null null null null))
          (:`OnRelease`
            (if (not (`self.Is Parrying`))
              (`self.K2_EndAbility`)))))
      (:`Is Not Valid`
        (`self.K2_EndAbility`)))
    (else
      (`self.K2_EndAbility`))))

(event `self.K2_OnEndAbility`
  (params (bWasCancelled :type Boolean))
  (`|ExecutionSequence`
    (:`then_0`
      (bind _returnvalue (message `BlockingActorInterface.GetBlockController` (`self.GetAvatarActorFromActorInfo`)))
      (`/Engine/EditorBlueprintResources/StandardMacros.IsValid` _returnvalue
        (:`Is Valid`
          (`BlockController.EndBlocking` _returnvalue))))
    (:`then_1`
      (`self.Clear Parry Effect Handles`)
      (set `self.Parried Target` null)
      (set `self.Is Parrying` false))))

(event `Manage Parry Window`
  (`KismetSystemLibrary.Delay` (`self.Get Parry Window Delay`))
  (bind _returnvalue (`ElectricCastleAbilitySystemLibrary.ApplyDurationEffectByTag` (`self.GetAvatarActorFromActorInfo`) (struct :`TagName` "Effect.State.Parrying") (`self.Get Parry Window Length`)))
  (set `self.Parry Handle` _returnvalue)
  (bind (_asynctaskproxy _payload) (`AbilityTask_WaitGameplayEvent.WaitGameplayEvent` (struct :`TagName` "Event.Montage.Common.ParryAttack") null true)
    (:`then`
      (`KismetSystemLibrary.Delay` (`self.Get Parry Window Length`))
      (`ElectricCastleAbilitySystemLibrary.RemoveGameplayEffect` (`self.GetAvatarActorFromActorInfo`) (`self.Parry Handle`) false true))
    (:`EventReceived`
      (`self.Handle Successful Parry` _payload))))

(event `Handle Successful Parry`
  (params (`Parry Payload` :type "GameplayEventData Structure"))
  (bind _returnvalue (`ElectricCastleAbilitySystemLibrary.GetRadialDamageOrigin` `Parry Payload_ContextHandle`))
  (set `self.Is Parrying` true)
  (bind _output_get (set `self.Parried Target` `Parry Payload_Instigator`))
  (message `CombatInterface.UpdateFacingTarget` `Parry Payload_Target` (`Actor.K2_GetActorLocation` _output_get))
  (bind _returnvalue_2 (`ElectricCastleAbilitySystemLibrary.ApplyInfiniteEffectByTag` (`self.GetAvatarActorFromActorInfo`) (struct :`TagName` "Effect.Block.Damage")))
  (set `self.Parry Invulnerability Handle` _returnvalue_2)
  (`GameplayStatics.PlaySoundAtLocation` (`self.Parry Sound`) _returnvalue (struct) 1.0 1.0 0.0 "/Game/Assets/Sounds/Abilities/FireBolt/att_InWorld.att_InWorld" null (`self.GetAvatarActorFromActorInfo`) null)
  (`NiagaraFunctionLibrary.SpawnSystemAtLocation` "/Game/Blueprints/Player/VFX/NS_SparkBurst_Parry.NS_SparkBurst_Parry" _returnvalue (struct) (1.0 1.0 1.0) true true "AutoRelease")
  (`AbilityTask_PlayMontageAndWait.CreatePlayMontageAndWaitProxy` "None" "/Game/MetaHumans/Common/Animation/Block/AM_Common_Parry.AM_Common_Parry"
    (:`then`
      (`AbilityTask_WaitGameplayEvent.WaitGameplayEvent` (struct :`TagName` "Event.Montage.Common.Parry.Land") null true
        (:`EventReceived`
          (bind _parried_target (`self.Parried Target`)
            (:`then`
              (message `CombatInterface.Stagger` _parried_target))
            (:`else`
              _))
          (`self.K2_EndAbility`))))
    (:`OnCompleted`
      (`self.K2_EndAbility` :!label _label))
    (:`OnBlendOut`
      (goto _label))
    (:`OnInterrupted`
      (goto _label))
    (:`OnCancelled`
      (goto _label))))

(event `Manage Block Hit`
  (bind (_asynctaskproxy _payload) (`AbilityTask_WaitGameplayEvent.WaitGameplayEvent` (struct :`TagName` "Event.Montage.Common.BlockAttack") null)
    (:`EventReceived`
      (`AbilityTask_PlayMontageAndWait.CreatePlayMontageAndWaitProxy` "None" "/Game/MetaHumans/Common/Animation/Block/AM_Common_BlockHit.AM_Common_BlockHit"
        (:`then`
          (bind _returnvalue (`ElectricCastleAbilitySystemLibrary.GetRadialDamageOrigin` (`.ContextHandle` (break `GameplayEventData` _payload))))
          (`GameplayStatics.PlaySoundAtLocation` (`self.Block Sound`) _returnvalue (struct) 1.0 1.0 0.0 "/Game/Assets/Sounds/Abilities/FireBolt/att_InWorld.att_InWorld" null (`self.GetAvatarActorFromActorInfo`) null)
          (`NiagaraFunctionLibrary.SpawnSystemAtLocation` "/Game/Blueprints/Player/VFX/NS_SparkBurst_White.NS_SparkBurst_White" _returnvalue (struct) (1.0 1.0 1.0) true true "AutoRelease"))))))

(fn `Clear Parry Effect Handles`
  (`ElectricCastleAbilitySystemLibrary.RemoveGameplayEffect` (`self.GetAvatarActorFromActorInfo`) (`self.Parry Handle`) false true)
  (`ElectricCastleAbilitySystemLibrary.RemoveGameplayEffect` (`self.GetAvatarActorFromActorInfo`) (`self.Parry Invulnerability Handle`) false true))

(fn `Get Parry Window Delay`
  (returns (Delay :type "Float (double-precision)"))
  (return (`AbilitySystemBlueprintLibrary.Conv_ScalableFloatToFloat` (`self.Parry Window Delay`) (`KismetMathLibrary.Conv_IntToDouble` (`self.GetAbilityLevel`)))))

(fn `Get Parry Window Length`
  (returns (Duration :type "Float (single-precision)"))
  (return (`AbilitySystemBlueprintLibrary.Conv_ScalableFloatToFloat` (`self.Parry Window`) (`KismetMathLibrary.Conv_IntToDouble` (`self.GetAbilityLevel`)))))