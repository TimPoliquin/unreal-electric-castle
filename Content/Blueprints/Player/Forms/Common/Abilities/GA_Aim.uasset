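; GA_Aim is a Gameplay Ability, shared by player forms, that keeps the avatar aiming while its input is held.
; On activation it commits, fetches the avatar's aim controller through GetAimControllerMessage and calls AimStart, or cancels if none is valid.
; A WaitInputRelease task then re-fetches the controller on release, calls AimEnd if it is valid, and ends the ability.
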(event `self.K2_ActivateAbility`
  (`self.K2_CommitAbility`)
  (bind _returnvalue (message `AimActorInterface.GetAimController` (`self.GetAvatarActorFromActorInfo`)))
  (`/Engine/EditorBlueprintResources/StandardMacros.IsValid` _returnvalue
    (:`Is Valid`
      (`AimController.AimStart` _returnvalue)
      (`AbilityTask_WaitInputRelease.WaitInputRelease` false
        (:`OnRelease`
          (bind _returnvalue_2 (message `AimActorInterface.GetAimController` (`self.GetAvatarActorFromActorInfo`)))
          (`/Engine/EditorBlueprintResources/StandardMacros.IsValid` _returnvalue_2
            (:`Is Valid`
              (`AimController.AimEnd` _returnvalue_2))
            (:`Is Not Valid`
              _))
          (`self.K2_EndAbility`))))
    (:`Is Not Valid`
      (`self.K2_CancelAbility`))))