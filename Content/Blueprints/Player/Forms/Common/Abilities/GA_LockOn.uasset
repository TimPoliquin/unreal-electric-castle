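; Gameplay ability that holds the avatar's lock-on state while its lock-on controller has a target.
; After committing, it applies the GE_LockedOn effect, or cancels if commit, controller or target is missing.
; It ends on input release, or a second press in toggle mode, or when lock-on level changes to None or Soft.
; Ending runs listener cleanup and removes the effect by its stored handle.
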(event `self.K2_ActivateAbility`
  (bind _returnvalue (`self.K2_CommitAbility`))
  (if _returnvalue
    (bind _returnvalue_2 (message `LockOnActor.GetLockOnController` (`self.GetAvatarActorFromActorInfo`)))
    (bind _output_get (set `self.Lock On Controller` _returnvalue_2))
    (`/Engine/EditorBlueprintResources/StandardMacros.IsValid` _output_get
      (:`Is Valid`
        (if (`LockOnController.HasLockOnTarget` _output_get)
          (bind _returnvalue_3 (`ElectricCastleAbilitySystemLibrary.ApplyBasicGameplayEffect` (`self.GetAvatarActorFromActorInfo`) "/Game/Blueprints/Player/Forms/Common/Effects/GE_LockedOn.GE_LockedOn_C"))
          (set `self.Lock On Effect Handle` _returnvalue_3)
          (`self.Wait for Lock On Input Release`)
          (`self.Listen for Lock On Release`)
          (else
            (`self.K2_CancelAbility`))))
      (:`Is Not Valid`
        (`self.K2_CancelAbility`)))
    (else
      (`self.K2_CancelAbility`))))

(event `Wait for Lock On Input Release`
  (if (`self.Lock On Input Toggle`)
    (`AbilityTask_WaitInputPress.WaitInputPress` false
      (:`OnPress`
        _))
    (else
      (`AbilityTask_WaitInputRelease.WaitInputRelease` false
        (:`OnRelease`
          _))))
  (`self.K2_EndAbility`))

(event `Listen for Lock On Release`
  (bind _lock_on_controller (`self.Lock On Controller`)
    (:`then`
      (add `LockOnController.OnLockOnLevelChanged` _lock_on_controller (delegate `OnLockOnTargetChanged_Event`)))
    (:`else`)))

(event `OnLockOnTargetChanged_Event`
  (params (Payload :type "LockOnTargetPayload Structure (by ref)"))
  (switch `ELockOnLevel` Payload_LockOnLevel
    (:`None`
      _)
    (:`Soft`
      _))
  (`self.K2_EndAbility`))

(event `Cleanup Event Listeners`
  (bind _lock_on_controller (`self.Lock On Controller`)
    (:`then`
      (remove `LockOnController.OnLockOnTargetChanged` _lock_on_controller (delegate `OnLockOnTargetChanged_Event`)))
    (:`else`)))

(event `self.K2_OnEndAbility`
  (params (bWasCancelled :type Boolean))
  (`|ExecutionSequence`
    (:`then_0`
      (`self.Cleanup Event Listeners`))
    (:`then_1`
      (`ElectricCastleAbilitySystemLibrary.RemoveGameplayEffect` (`self.GetAvatarActorFromActorInfo`) (`self.Lock On Effect Handle`) false true))))