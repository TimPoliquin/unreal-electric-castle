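; Gameplay ability for the Barbarian form's charged heavy attack, where hold time scales the damage dealt.
; It plays the montage's Start section, waits for the Hold gameplay event, then waits for input release to play the Release section.
; Normalized hold time samples a curve for the damage multiplier, applied to each target reported by Hit events.
; The ability ends with the release montage and resets the multiplier.
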(event `self.K2_OnEndAbility`
  (params (bWasCancelled :type Boolean))
  (set `self.Hold Time Damage Multipler` 0.0))

(event `self.K2_ActivateAbility`
  (bind _returnvalue (`self.K2_CommitAbility`))
  (if _returnvalue
    (`AbilityTask_PlayMontageAndWait.CreatePlayMontageAndWaitProxy` "Barbarian Heavy Attack" "/Game/MetaHumans/MHC_Barbarian/Animations/Combat/AM_Barbarian_Attack_Heavy.AM_Barbarian_Attack_Heavy" 1.0 "Start"
      (:`then`
        (`AbilityTask_WaitGameplayEvent.WaitGameplayEvent` (struct :`TagName` "Event.Montage.Barbarian.Secondary.Hold") null true
          (:`EventReceived`
            (bind (_asynctaskproxy _timeheld) (`AbilityTask_WaitInputRelease.WaitInputRelease` true)
              (:`OnRelease`
                (`self.Calculate Hold Time Damage Multipler` _timeheld)
                (`AbilityTask_PlayMontageAndWait.CreatePlayMontageAndWaitProxy` "None" "/Game/MetaHumans/MHC_Barbarian/Animations/Combat/AM_Barbarian_Attack_Heavy.AM_Barbarian_Attack_Heavy" 1.0 "Release"
                  (:`then`
                    (bind (_asynctaskproxy_2 _payload) (`AbilityTask_WaitGameplayEvent.WaitGameplayEvent` (struct :`TagName` "Event.Montage.Barbarian.Secondary.Hit") null)
                      (:`EventReceived`
                        (`self.Handle Hit Target` _payload))))
                  (:`OnCompleted`
                    (`self.K2_EndAbility` :!label _label))
                  (:`OnBlendOut`
                    (goto _label))
                  (:`OnInterrupted`
                    (goto _label))
                  (:`OnCancelled`
                    (goto _label)))))))))
    (else
      (`self.K2_EndAbility`))))

(event `Handle Hit Target`
  (params (Payload :type "GameplayEventData Structure"))
  (bind (_eventtag _instigator _target _optionalobject _optionalobject2 _contexthandle) (break `GameplayEventData` Payload))
  (`self.DamageTarget` _target (`.ImpactPoint` (`GameplayStatics.BreakHitResult` (`AbilitySystemBlueprintLibrary.EffectContextGetHitResult` _contexthandle))) _eventtag (`self.Hold Time Damage Multipler`)))

(fn `Calculate Hold Time Damage Multipler`
  (params (`Hold Time` :type "Float (double-precision)"))
  (set `self.Hold Time Damage Multipler` (`KismetMathLibrary.GetRuntimeFloatCurveValue` (`self.Hold Time Damage Multiplier Curve`) (`KismetMathLibrary.SafeDivide` `Hold Time` (`self.Max Hold Time`)) 0.5)))