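; Highlander primary attack ability, extending a parent combo ability with a dagger flip during the attack montage.
; After the parent's combo montage event handling, the server waits for the Highlander Flip gameplay event.
; On that event it finds the right dagger mesh by socket tag through the avatar weapon's socket manager and, if valid, adds a 180-degree relative rotation.
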(event `self.Wait for Combo Montage Event`
  (`parent.Wait for Combo Montage Event`)
  (`self.K2_HasAuthority`
    (:`True`
      (`AbilityTask_WaitGameplayEvent.WaitGameplayEvent` (struct :`TagName` "Event.Montage.Highlander.Flip") null
        (:`EventReceived`
          (bind _returnvalue (message `CombatInterface.GetWeapon` (`self.GetAvatarActorFromActorInfo`)))
          (bind _returnvalue_2 (message `SocketManagerActor.GetSocketManagerComponent` _returnvalue))
          (bind _returnvalue_3 (`SocketManagerComponent.GetMeshBySocketTag` _returnvalue_2 (`BlueprintGameplayTagLibrary.MakeLiteralGameplayTag` (struct :`TagName` "Combat.Socket.Weapon.Dagger.Right"))))
          (`/Engine/EditorBlueprintResources/StandardMacros.IsValid` _returnvalue_3
            (:`Is Valid`
              (`SceneComponent.K2_AddRelativeRotation` _returnvalue_3 (struct :`Pitch` 180.0) false false))))))))