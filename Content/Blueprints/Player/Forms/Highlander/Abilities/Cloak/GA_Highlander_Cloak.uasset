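; Gameplay ability that cloaks the player's Highlander form until input is pressed again, then ends the cloak through the avatar's cloak component.
; On activation it commits, plays the cloak montage and updates the avatar's facing target with its own location.
; A montage gameplay event triggers StartCloak on the component.
; An infinite lock-on block effect is applied during the montage and removed only when it completes.
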(event `self.K2_OnEndAbility`
  (params (bWasCancelled :type Boolean))
  (`|ExecutionSequence`
    (:`then_0`
      (bind _returnvalue (message `CloakActorInterface.GetCloakComponent` (`self.GetAvatarActorFromActorInfo`)))
      (`/Engine/EditorBlueprintResources/StandardMacros.IsValid` _returnvalue
        (:`Is Valid`
          (`CloakComponent.EndCloak` _returnvalue))))))

(event `self.K2_ActivateAbility`
  (bind _returnvalue (`self.GetAvatarActorFromActorInfo`))
  (bind _returnvalue_2 (`self.K2_CommitAbility`))
  (if _returnvalue_2
    (`self.Execute`)
    (message `CombatInterface.UpdateFacingTarget` _returnvalue (`Actor.K2_GetActorLocation` _returnvalue))
    (`AbilityTask_WaitInputPress.WaitInputPress` false
      (:`OnPress`
        (`self.K2_EndAbility`)))))

(event `Execute`
  (`AbilityTask_PlayMontageAndWait.CreatePlayMontageAndWaitProxy` "None" "/Game/MetaHumans/MHC_Highlander/Animations/Ability/AM_Highlander_Cloak.AM_Highlander_Cloak"
    (:`then`
      (`AbilityTask_WaitGameplayEvent.WaitGameplayEvent` (struct :`TagName` "Event.Montage.Highlander.Cloak") null
        (:`then`
          (bind _returnvalue (`ElectricCastleAbilitySystemLibrary.ApplyInfiniteEffectByTag` (`self.GetAvatarActorFromActorInfo`) (struct :`TagName` "Player.Block.LockOn"))))
        (:`EventReceived`
          (`self.Apply Cloak Effect`))))
    (:`OnCompleted`
      (`ElectricCastleAbilitySystemLibrary.RemoveGameplayEffect` (`self.GetAvatarActorFromActorInfo`) _returnvalue false true))))

(event `Apply Cloak Effect`
  (`|ExecutionSequence`
    (:`then_0`
      (bind _returnvalue (message `CloakActorInterface.GetCloakComponent` (`self.GetAvatarActorFromActorInfo`)))
      (`/Engine/EditorBlueprintResources/StandardMacros.IsValid` _returnvalue
        (:`Is Valid`
          (`CloakComponent.StartCloak` _returnvalue))))))