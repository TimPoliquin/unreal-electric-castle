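; Primary attack ability for the Native player form: a draw-and-release bow shot.
; On activation it commits, optionally faces the target under the mouse, then plays the draw montage section while the server attaches a collision-disabled arrow to the right hand.
; Releasing input plays the fire section, where the server removes the aiming effect and detaches and releases the arrow.
; A new press or the fire montage finishing ends the ability.
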(event `self.K2_ActivateAbility`
  (bind _returnvalue (`self.K2_CommitAbility`))
  (if _returnvalue
    (if (`self.ShouldSetMotionTarget`)
      (bind (_asynctaskproxy _datahandle) (`TargetDataUnderMouse.CreateTargetDataUnderMouse`)
        (:`HasMouseTarget`
          (bind _returnvalue_2 (`AbilitySystemBlueprintLibrary.GetHitResultFromTargetData` _datahandle))
          (`self.FaceHitTarget` _returnvalue_2)
          (set `self.Target Actor` (`.HitActor` (`GameplayStatics.BreakHitResult` _returnvalue_2)))
          (`self.Execute Attack`))
        (:`HasNoTarget`
          (message `CombatInterface.ClearFacingTarget` (`self.GetAvatarActorFromActorInfo`) :!label _label)
          (`self.Execute Attack`)))
      (else
        (goto _label)))
    (else
      (`self.K2_CancelAbility`))))

(event `Execute Attack`
  (`AbilityTask_PlayMontageAndWait.CreatePlayMontageAndWaitProxy` "None" (`self.Montage to Play`) 1.0 "Combo.01"
    (:`then`
      (`|ExecutionSequence`
        (:`then_0`
          (`AbilityTask_WaitInputRelease.WaitInputRelease` true
            (:`OnRelease`
              (`self.Fire!`))))
        (:`then_1`
          (`self.K2_HasAuthority`
            (:`True`
              (bind _projectile (`self.Create Projectile`))
              (set `self.Projectile` _projectile))))))
    (:`OnCancelled`
      (`self.K2_EndAbility`))))

(event `Fire!`
  (`AbilityTask_PlayMontageAndWait.CreatePlayMontageAndWaitProxy` "None" (`self.Montage to Play`) 1.0 "Combo.03"
    (:`then`
      (`self.K2_HasAuthority`
        (:`True`
          (`self.Remove Aim Effect`)
          (bind _projectile (`self.Projectile`)
            (:`then`
              (`Actor.K2_DetachFromActor` _projectile "KeepWorld" "KeepWorld" "KeepWorld")
              (bind _asbp_native_primary_arrow (cast `/Game/Blueprints/Player/Forms/Native/Abilities/BP_Native_Primary_Arrow` (`self.Projectile`)))
              (`ArrowProjectile.Release` _asbp_native_primary_arrow)
              (`self.Cleanup`)
              (`AbilityTask_WaitInputPress.WaitInputPress` false
                (:`OnPress`
                  (`self.K2_EndAbility`))))
            (:`else`
              (`KismetSystemLibrary.PrintString` "No projectile???")
              (`self.K2_EndAbility`))))))
    (:`OnCompleted`
      (`self.K2_EndAbility` :!label _label_2))
    (:`OnBlendOut`
      (goto _label_2))
    (:`OnInterrupted`
      (goto _label_2))
    (:`OnCancelled`
      (goto _label_2))))

(event `Remove Aim Effect`
  (`ElectricCastleAbilitySystemLibrary.RemoveGameplayEffect` (`self.GetAvatarActorFromActorInfo`) (`self.Aiming Effect Handle`) false))

(event `Cleanup`
  (set `self.Projectile` null)
  (bind _async_task (`self.Async Task`)
    (:`then`
      (`GameplayTask.EndTask` _async_task)
      (set `self.Target Actor` null))
    (:`else`)))

(fn `Create Projectile`
  (returns (Projectile :type "ProjectileActor Object Reference"))
  (locals (`Local Projectile` :type "ArrowProjectile Object Reference"))
  (bind _ascharacter (cast `Character` (`self.GetAvatarActorFromActorInfo`))
    (:`then`
      (bind _returnvalue (`self.SpawnProjectile_Basic`))
      (bind _asarrow_projectile (cast `ArrowProjectile` _returnvalue)
        (:`then`
          (bind _output_get (set `local.Local Projectile` _asarrow_projectile)))
        (:`CastFailed`
          _))
      (`Actor.K2_AttachToComponent` _output_get (`Character.Mesh` _ascharacter) "Socket_Hand_Right" "SnapToTarget" "KeepWorld" "KeepRelative" false)
      (`/Engine/EditorBlueprintResources/StandardMacros.IsValid` (`local.Local Projectile`)
        (:`Is Valid`
          (`PrimitiveComponent.SetCollisionEnabled` (`ProjectileActor.CollisionComponent` (`local.Local Projectile`)) "NoCollision")
          (set `ArrowProjectile.Pitch` (`self.Pitch`) (`local.Local Projectile`)))
        (:`Is Not Valid`
          _)))
    (:`CastFailed`
      _))
  (return (`local.Local Projectile`)))