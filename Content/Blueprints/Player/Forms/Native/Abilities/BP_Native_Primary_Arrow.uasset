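; Pooled arrow projectile for the Native player form's primary ability, extending a parent class that supplies the firing and pool logic.
; Each override calls its parent first, then manages the arrow's effects.
; Firing activates the head effect without a reset, while pool retrieval and return deactivate both head and trail effects.
; The trail effect is never activated in this Blueprint.
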(event `self.OnPool_FinishRetrieve`
  (params (Payload :type "SpawnPoolEventPayload Structure (by ref)"))
  (`parent.OnPool_FinishRetrieve` Payload)
  (`ActorComponent.Deactivate` (`self.Head Effect`))
  (`ActorComponent.Deactivate` (`self.TrailFX`)))

(event `self.OnPool_Returned`
  (params (Payload :type "SpawnPoolEventPayload Structure (by ref)"))
  (`parent.OnPool_Returned` Payload)
  (`ActorComponent.Deactivate` (`self.Head Effect`))
  (`ActorComponent.Deactivate` (`self.TrailFX`)))

(event `self.Fire`
  (`parent.Fire`)
  (`ActorComponent.Activate` (`self.Head Effect`) false))

(fn `UserConstructionScript`)