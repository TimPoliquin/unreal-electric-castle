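; Futureman's Chrono Shift gameplay ability changes global time dilation while giving the avatar the inverse, keeping it at normal speed.
; Activation applies level-scaled magnitude, motion blur and a tagged duration effect.
; It ends on a second press or after a delay multiplied by magnitude to compensate for dilation, then resets time and blur and removes the effect.
; ApplyBlurEffect is never called and looks unfinished.
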(event `self.K2_ActivateAbility`
  (bind _returnvalue (`self.K2_CommitAbility`))
  (if _returnvalue
    (bind _current_magnitude (`self.Apply Time Dilation`))
    (`|ExecutionSequence`
      (:`then_0`
        (`AbilityTask_WaitInputPress.WaitInputPress` false
          (:`OnPress`
            (`self.K2_EndAbility`))))
      (:`then_1`
        (`KismetSystemLibrary.Delay` (`self.Calculate Delay` _current_magnitude))
        (`self.K2_EndAbility`)))))

(event `self.K2_OnEndAbility`
  (params (bWasCancelled :type Boolean))
  (`GameplayStatics.SetGlobalTimeDilation` 1.0)
  (set `Actor.CustomTimeDilation` 1.0 (`self.GetAvatarActorFromActorInfo`))
  (`PostProcessUtils.SetMotionBlurAmount` (`self.GetAvatarActorFromActorInfo`))
  (`ElectricCastleAbilitySystemLibrary.RemoveGameplayEffect` (`self.GetAvatarActorFromActorInfo`) (`self.ChronoShiftEffect`) false))

(fn `Apply Blur Effect`
  (params (BlurAmount :type "Float (double-precision)" :default 0.5))
  (bind _outactors (`GameplayStatics.GetAllActorsOfClass` "/Script/Engine.PostProcessVolume"))
  (for _array_element _outactors
    (set `PostProcessVolume.Settings` (struct) _array_element)))

(fn `Apply Time Dilation`
  (returns (`Current Magnitude` :type "Float (double-precision)"))
  (locals (`Local Magnitude` :type "Float (single-precision)" :default 0.0))
  (bind _output_get (set `local.Local Magnitude` (`AbilitySystemBlueprintLibrary.Conv_ScalableFloatToFloat` (`self.Magnitude`) (`KismetMathLibrary.Conv_IntToDouble` (`self.GetAbilityLevel`)))))
  (`GameplayStatics.SetGlobalTimeDilation` _output_get)
  (set `Actor.CustomTimeDilation` (/ 1.0 _output_get) (`self.GetAvatarActorFromActorInfo`))
  (`PostProcessUtils.SetMotionBlurAmount` (`self.GetAvatarActorFromActorInfo`) (`self.Blur Amount`))
  (bind _returnvalue (`ElectricCastleAbilitySystemLibrary.ApplyDurationEffectByTag` (`self.GetAvatarActorFromActorInfo`) (struct :`TagName` "Effect.State.ChronoShift") (`AbilitySystemBlueprintLibrary.Conv_ScalableFloatToFloat` (`self.Duration`) (`KismetMathLibrary.Conv_IntToDouble` (`self.GetAbilityLevel`))) (`self.GetAbilityLevel`)))
  (set `self.ChronoShiftEffect` _returnvalue)
  (return (`local.Local Magnitude`)))

(fn `Calculate Delay`
  (params (`Current Magnitude` :type "Float (double-precision)"))
  (returns (`Delay Duration` :type "Float (double-precision)"))
  (return (* (`AbilitySystemBlueprintLibrary.Conv_ScalableFloatToFloat` (`self.Duration`) (`KismetMathLibrary.Conv_IntToDouble` (`self.GetAbilityLevel`))) (`local.Current Magnitude`))))