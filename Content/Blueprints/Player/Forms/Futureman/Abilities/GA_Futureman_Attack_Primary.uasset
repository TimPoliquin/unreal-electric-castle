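; Futureman's primary attack ability, which fires laser projectiles as part of a combo attack.
; When an attack event supplies a combo config, it resolves the montage hit location and, on success, spawns a projectile there facing the aim target.
; Projectiles come from an actor pool through deferred acquire and finalize, receiving damage parameters, explosion damage effect, owner and instigator before finalization.
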(event `self.Attack Targets at Location`
  (params (Targets :type "Array of Actor Object Reference (by ref)") (ImpactLocation :type "Vector Structure (by ref)") (`Combo Config` :type "ComboAbilityConfig Structure (by ref)"))
  (bind (_combohitlocation _returnvalue) (`self.GetComboMontageHitLocation` `Combo Config`))
  (set `self.Combo Hit Location` _combohitlocation)
  (if _returnvalue
    (`self.Create Projectile`)))

(fn `Create Projectile`
  (locals (Projectile :type "/Game/Blueprints/Player/Forms/Futureman/Abilities/BP_LaserProjectile Object Reference"))
  (bind _outactor (`PoolActorFunctionLibrary.AcquirePooledActorDeferred` "/Game/Blueprints/Player/Forms/Futureman/Abilities/BP_LaserProjectile.BP_LaserProjectile_C"))
  (set `local.Projectile` _outactor)
  (set `ProjectileActor.DamageEffectParams` (`self.MakeDamageEffectParamsFromClassDefaults` null) (`local.Projectile`))
  (set `ProjectileActor.ExplosionDamageEffectClass` "/Game/Blueprints/AbilitySystem/GameplayEffects/GE_Damage.GE_Damage_C" (`local.Projectile`))
  (`Actor.SetOwner` (`local.Projectile`) (`self.GetAvatarActorFromActorInfo`))
  (set `Actor.Instigator` (cast `Pawn` (`self.GetAvatarActorFromActorInfo`) :!pure true) (`local.Projectile`))
  (`PoolActorFunctionLibrary.FinalizePooledActor` (`local.Projectile`) (`KismetMathLibrary.MakeTransform` (`self.Combo Hit Location`) (`self.CalculateSpawnRotationFacingAimTarget` (`self.Combo Hit Location`)))))