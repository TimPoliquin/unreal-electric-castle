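; Futureman's Chrono Shift ability, which applies time dilation to the world and the inverse to the player for a level-scaled duration.
; A montage event triggers the shift after a short delay, with movement blocked during the montage.
; The server sets dilation and gameplay effects, while motion blur also changes.
; The ability ends on input press or a timer scaled by the dilation, restoring time and resetting blur.
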(event `self.K2_ActivateAbility`
  (bind _returnvalue (`self.K2_CommitAbility`))
  (if _returnvalue
    (`AbilityTask_PlayMontageAndWait.CreatePlayMontageAndWaitProxy` "None" "/Game/MetaHumans/MHC_Futureman/Animations/Combat/AM_Futureman_ChronoShift.AM_Futureman_ChronoShift"
      (:`then`
        (`AbilityTask_WaitGameplayEvent.WaitGameplayEvent` (struct :`TagName` "Event.Montage.Futureman.ChronoShift.Activate") null
          (:`then`
            (`self.Apply Block Movement Effect`))
          (:`EventReceived`
            (`KismetSystemLibrary.Delay` 0.5)
            (`self.Execute`))))
      (:`OnCompleted`
        (`self.Remove Block Movement Effect` :!label _label))
      (:`OnBlendOut`
        (goto _label))
      (:`OnInterrupted`
        (goto _label))
      (:`OnCancelled`
        (goto _label)))))

(event `Execute`
  (bind _current_magnitude (`self.Apply Time Dilation`))
  (`|ExecutionSequence`
    (:`then_0`
      (`AbilityTask_WaitInputPress.WaitInputPress` false
        (:`OnPress`
          (`self.K2_EndAbility`))))
    (:`then_1`
      (`KismetSystemLibrary.Delay` (`self.Calculate Delay` _current_magnitude))
      (`self.K2_EndAbility`))))

(event `self.K2_OnEndAbility`
  (params (bWasCancelled :type Boolean))
  (`|ExecutionSequence`
    (:`then_0`
      (`self.K2_HasAuthority`
        (:`True`
          (`ElectricCastleAbilitySystemLibrary.RemoveGameplayEffect` (`self.GetAvatarActorFromActorInfo`) (`self.ChronoShiftEffect`) false)
          (`PlayerManager.SetTimeDilation` (subsystem `PlayerManager`) 1.0 1.0)
          (`self.Remove Block Movement Effect`))))
    (:`then_1`
      (`PostProcessUtils.SetMotionBlurAmount` (`self.GetAvatarActorFromActorInfo`)))))

(fn `Apply Block Movement Effect`
  (`self.K2_HasAuthority`
    (:`True`
      (bind _returnvalue (`ElectricCastleAbilitySystemLibrary.ApplyInfiniteEffectByTag` (`self.GetAvatarActorFromActorInfo`) (struct :`TagName` "Player.Block.Movement")))
      (set `self.Block Movement Effect` _returnvalue))))

(fn `Apply Blur Effect`
  (params (BlurAmount :type "Float (double-precision)" :default 0.5))
  (bind _outactors (`GameplayStatics.GetAllActorsOfClass` "/Script/Engine.PostProcessVolume"))
  (for _array_element _outactors
    (set `PostProcessVolume.Settings` (struct) _array_element)))

(fn `Apply Time Dilation`
  (returns (`Current Magnitude` :type "Float (double-precision)"))
  (locals (`Local Magnitude` :type "Float (single-precision)" :default 0.0))
  (bind _output_get (set `local.Local Magnitude` (`AbilitySystemBlueprintLibrary.Conv_ScalableFloatToFloat` (`self.Magnitude`) (`KismetMathLibrary.Conv_IntToDouble` (`self.GetAbilityLevel`)))))
  (`|ExecutionSequence`
    (:`then_0`
      (`self.K2_HasAuthority`
        (:`True`
          (`PlayerManager.SetTimeDilation` (subsystem `PlayerManager`) _output_get (/ 1.0 (`local.Local Magnitude`)))
          (bind _returnvalue (`ElectricCastleAbilitySystemLibrary.ApplyDurationEffectByTag` (`self.GetAvatarActorFromActorInfo`) (struct :`TagName` "Effect.State.ChronoShift") (`AbilitySystemBlueprintLibrary.Conv_ScalableFloatToFloat` (`self.Duration`) (`KismetMathLibrary.Conv_IntToDouble` (`self.GetAbilityLevel`))) (`self.GetAbilityLevel`)))
          (set `self.ChronoShiftEffect` _returnvalue))))
    (:`then_1`
      (`PostProcessUtils.SetMotionBlurAmount` (`self.GetAvatarActorFromActorInfo`) (`self.Blur Amount`)))
    (:`then_2`
      (return (`local.Local Magnitude`)))))

(fn `Calculate Delay`
  (params (`Current Magnitude` :type "Float (double-precision)"))
  (returns (`Delay Duration` :type "Float (double-precision)"))
  (return (* (`AbilitySystemBlueprintLibrary.Conv_ScalableFloatToFloat` (`self.Duration`) (`KismetMathLibrary.Conv_IntToDouble` (`self.GetAbilityLevel`))) (`local.Current Magnitude`))))

(fn `Remove Block Movement Effect`
  (bind _block_movement_effect (`self.Block Movement Effect`))
  (bind _returnvalue (`AbilitySystemBlueprintLibrary.IsActiveGameplayEffectHandleValid` _block_movement_effect))
  (if _returnvalue
    (`ElectricCastleAbilitySystemLibrary.RemoveGameplayEffect` (`self.GetAvatarActorFromActorInfo`) _block_movement_effect false)))