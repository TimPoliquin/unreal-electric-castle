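; Futureman's Charge Shot gameplay ability: holds a projectile that gains power while input is held, then fires it on release.
; A montage event triggers acquiring a pooled projectile, attached to the avatar between both blaster tips with collision disabled.
; A recursive delay loop raises its power level, using scalable floats for the ability-level cap and per-charge delay.
; Release plays the end montage, rotates the projectile toward the aim target, fires and ends the ability.
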(event `self.K2_OnEndAbility`
  (params (bWasCancelled :type Boolean))
  (set `self.Projectile` null)
  (set `self.Current Charge Level` 1))

(event `self.K2_ActivateAbility`
  (bind _returnvalue (`self.K2_CommitAbility`))
  (if _returnvalue
    (`AbilityTask_PlayMontageAndWait.CreatePlayMontageAndWaitProxy` "Futureman_ChargeShot_Start" "/Game/MetaHumans/MHC_Futureman/Animations/Combat/ChargeShot/AM_Futureman_ChargeShot.AM_Futureman_ChargeShot" 1.0 "Start"
      (:`then`
        (bind (_asynctaskproxy _payload) (`AbilityTask_WaitGameplayEvent.WaitGameplayEvent` (struct :`TagName` "Event.Montage.Futureman.ChargeShot.Ready") null true)
          (:`EventReceived`
            (`self.Event Handle Charge Shot Ready` _payload)))))
    (else
      (`self.K2_EndAbility`))))

(event `Event Handle Charge Shot Ready`
  (params (Payload :type "GameplayEventData Structure"))
  (bind _returnvalue (`self.Spawn Projectile`))
  (set `self.Projectile` _returnvalue)
  (`self.Prepare Charge Up`)
  (`AbilityTask_WaitInputRelease.WaitInputRelease` true
    (:`OnRelease`
      (`AbilityTask_PlayMontageAndWait.CreatePlayMontageAndWaitProxy` "Futureman_ChargeShot_End" "/Game/MetaHumans/MHC_Futureman/Animations/Combat/ChargeShot/AM_Futureman_ChargeShot.AM_Futureman_ChargeShot" 1.0 "End"
        (:`then`
          (`|ExecutionSequence`
            (:`then_0`
              (`self.Projectile`
                (:`then`
                  (`self.RotateTowardAvatarActorAimTarget` (`self.Projectile`))
                  (`ProjectileActor.Fire` (`self.Projectile`))
                  (set `self.Projectile` null))
                (:`else`)))
            (:`then_1`
              (`self.K2_EndAbility` :!label _label))))
        (:`OnCompleted`
          (goto _label))
        (:`OnBlendOut`
          (goto _label))
        (:`OnInterrupted`
          (goto _label))
        (:`OnCancelled`
          (goto _label))))))

(event `Prepare Charge Up`
  (if (< (`self.Current Charge Level`) (`AbilitySystemBlueprintLibrary.Conv_ScalableFloatToFloat` (`self.Charge Up Levels`) (`KismetMathLibrary.Conv_IntToDouble` (`self.GetAbilityLevel`))))
    (`KismetSystemLibrary.Delay` (`AbilitySystemBlueprintLibrary.Conv_ScalableFloatToFloat` (`self.Charge Up Levels Delay`) (`KismetMathLibrary.Conv_IntToDouble` (`self.Current Charge Level`))))
    (`self.Projectile`
      (:`then`
        (`/Engine/EditorBlueprintResources/StandardMacros.IncrementInt` (`self.Current Charge Level`)
          (:`  `
            (`/Game/Blueprints/Player/Forms/Futureman/Abilities/ChargeShot/BP_ChargeShot_Projectile.Set Power Level` (`self.Projectile`) (`self.Current Charge Level`))
            (`self.Prepare Charge Up`))))
      (:`else`))))

(fn `Spawn Projectile`
  (returns (ReturnValue :type "/Game/Blueprints/Player/Forms/Futureman/Abilities/ChargeShot/BP_ChargeShot_Projectile Object Reference"))
  (locals (`Local Projectile` :type "/Game/Blueprints/Player/Forms/Futureman/Abilities/ChargeShot/BP_ChargeShot_Projectile Object Reference") (`Projectile Spawn Location` :type "Vector Structure" :default (0.0 0.0 0.0)))
  (bind _outactor (`PoolActorFunctionLibrary.AcquirePooledActorDeferred` "/Game/Blueprints/Player/Forms/Futureman/Abilities/ChargeShot/BP_ChargeShot_Projectile.BP_ChargeShot_Projectile_C"))
  (bind _output_get (set `local.Local Projectile` _outactor))
  (`Actor.K2_AttachToActor` _output_get (`self.GetAvatarActorFromActorInfo`) "None" "KeepRelative" "KeepRelative" "KeepRelative" true)
  (bind _output_get_2 (set `local.Projectile Spawn Location` (+ (/ (+ (`self.GetAvatarActorSocketLocation` (`BlueprintGameplayTagLibrary.MakeLiteralGameplayTag` (struct :`TagName` "Combat.Socket.Weapon.Blaster.Left.Tip")) true) (`self.GetAvatarActorSocketLocation` (`BlueprintGameplayTagLibrary.MakeLiteralGameplayTag` (struct :`TagName` "Combat.Socket.Weapon.Blaster.Right.Tip")) true)) 2.0) (* (`self.GetAvatarActorForwardVector`) 10.0))))
  (`Actor.K2_SetActorRelativeLocation` (`local.Local Projectile`) (`KismetMathLibrary.InverseTransformLocation` (`Actor.GetTransform` (`self.GetAvatarActorFromActorInfo`)) _output_get_2) false true)
  (set `ProjectileActor.DamageEffectParams` (`self.MakeDamageEffectParamsFromClassDefaults` null) (`local.Local Projectile`))
  (`self.SetOwnerAndInstigator` (`local.Local Projectile`))
  (set `/Game/Blueprints/Player/Forms/Futureman/Abilities/ChargeShot/BP_ChargeShot_Projectile.Initial Power Level` 1 (`local.Local Projectile`))
  (set `/Game/Blueprints/Player/Forms/Futureman/Abilities/ChargeShot/BP_ChargeShot_Projectile.Damage Magnitude` (`.DamageMagnitude` (break `ElectricCastleDamageConfig` (`self.DamageConfig`))) (`local.Local Projectile`))
  (`PoolActorFunctionLibrary.FinalizePooledActor` (`local.Local Projectile`) (`KismetMathLibrary.MakeTransform` (`local.Projectile Spawn Location`)))
  (`PrimitiveComponent.SetCollisionEnabled` (`ProjectileActor.CollisionComponent` (`local.Local Projectile`)) "NoCollision")
  (return (`local.Local Projectile`)))