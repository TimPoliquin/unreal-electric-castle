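; Pooled projectile for Futureman's Charge Shot ability, with looks, sound and damage that scale with its power level.
; On pool retrieval it applies the initial power level; on return it deactivates effects and clears that level.
; Setting a level applies that entry of a per-level config to mesh, charge-up and fizzle effects, and overrides damage from a scalable float.
; Firing plays a release sound at its location.
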(event `self.OnPool_FinishRetrieve`
  (params (Payload :type "SpawnPoolEventPayload Structure (by ref)"))
  (`parent.OnPool_FinishRetrieve` Payload)
  (`self.Set Power Level` (`self.Initial Power Level`)))

(event `self.OnPool_Returned`
  (params (Payload :type "SpawnPoolEventPayload Structure (by ref)"))
  (`parent.OnPool_Returned` Payload)
  (`ActorComponent.Deactivate` (`self.Charge Up FX`))
  (`ActorComponent.Deactivate` (`self.Fizzle FX`))
  (`ActorComponent.Deactivate` (`self.Charge Up SFX`))
  (`ActorComponent.Deactivate` (`self.Fizzle SFX`))
  (set `self.Initial Power Level` 0))

(event `Set Power Level`
  (params (`In Power Level` :type Integer))
  (set `self.Power Level` `In Power Level`)
  (`self.Set Power Level Visible Nodes`)
  (`self.OverrideDamageMagnitude` (`AbilitySystemBlueprintLibrary.Conv_ScalableFloatToFloat` (`self.Damage Magnitude`) (`KismetMathLibrary.Conv_IntToDouble` (`self.Power Level`)))))

(event `self.Fire`
  (`parent.Fire`)
  (`GameplayStatics.PlaySoundAtLocation` "/Game/Assets/Sounds/Abilities/Futureman/ChargeShot/sfx_Futureman_ChargeShot_Release.sfx_Futureman_ChargeShot_Release" (`self.K2_GetActorLocation`) (struct) 1.0 1.0 0.0 "/Game/Assets/Sounds/Abilities/FireBolt/att_InWorld.att_InWorld" null self null))

(fn `Set Power Level Visible Nodes`
  (locals (`Current Config` :type "/Game/Blueprints/Player/Forms/Futureman/Abilities/ChargeShot/F_Futureman_ChargeShot_LevelConfig Structure"))
  (bind (_current_config_chargeeffectsystem _current_config_chargeeffectsound _current_config_chargeeffectsoundvolumemultiplier _current_config_staticeffectsystem _current_config_staticsound _current_config_staticsoundvolumemultiplier) (break `/Game/Blueprints/Player/Forms/Futureman/Abilities/ChargeShot/F_Futureman_ChargeShot_LevelConfig` (`local.Current Config`)))
  (bind (_current_config_chargeeffectsystem_2 _current_config_chargeeffectsound_2 _current_config_chargeeffectsoundvolumemultiplier_2) (break `/Game/Blueprints/Player/Forms/Futureman/Abilities/ChargeShot/F_Futureman_ChargeShot_LevelConfig` (`local.Current Config`)))
  (bind (_current_config_chargeeffectsystem_3 _current_config_chargeeffectsound_3 _current_config_chargeeffectsoundvolumemultiplier_3 _current_config_staticeffectsystem_2 _current_config_staticsound_2 _current_config_staticsoundvolumemultiplier_2 _current_config_mesh _current_config_meshscale _current_config_meshmaterial) (break `/Game/Blueprints/Player/Forms/Futureman/Abilities/ChargeShot/F_Futureman_ChargeShot_LevelConfig` (`local.Current Config`)))
  (set `local.Current Config` (`|GetArrayItem` (`self.Charge Level Configuration`) (- (`self.Power Level`) 1)))
  (`|ExecutionSequence`
    (:`then_0`
      ; Set Mesh Values
      (`StaticMeshComponent.SetStaticMesh` (`self.Mesh`) _current_config_mesh)
      (`SceneComponent.SetWorldScale3D` (`self.Mesh`) _current_config_meshscale)
      (`PrimitiveComponent.SetMaterial` (`self.Mesh`) 0 _current_config_meshmaterial)
      (`SceneComponent.SetHiddenInGame` (`self.Mesh`) false true))
    (:`then_1`
      ; Set Charge FX/SFX
      (`NiagaraComponent.SetAsset` (`self.Charge Up FX`) _current_config_chargeeffectsystem_2 true)
      (`ActorComponent.Activate` (`self.Charge Up FX`) true)
      (`AudioComponent.SetSound` (`self.Charge Up SFX`) _current_config_chargeeffectsound_2)
      (`AudioComponent.SetVolumeMultiplier` (`self.Charge Up SFX`) _current_config_chargeeffectsoundvolumemultiplier_2)
      (`ActorComponent.Activate` (`self.Charge Up SFX`) true)
      (`AudioComponent.Play` (`self.Charge Up SFX`) 0.0))
    (:`then_2`
      ; Set Fizzle FX/SFX
      (`NiagaraComponent.SetAsset` (`self.Fizzle FX`) _current_config_staticeffectsystem true)
      (`ActorComponent.Activate` (`self.Fizzle FX`) true)
      (`AudioComponent.SetSound` (`self.Fizzle SFX`) _current_config_staticsound)
      (`AudioComponent.SetVolumeMultiplier` (`self.Fizzle SFX`) _current_config_staticsoundvolumemultiplier)
      (`ActorComponent.Activate` (`self.Fizzle SFX`) true)
      (`AudioComponent.Play` (`self.Fizzle SFX`) 0.0))))

(fn `UserConstructionScript`)