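; Gameplay ability for the Egyptian form's primary attack, which fires a beam.
; On commit it tracks input release for hold time and, when motion targeting applies, faces the target under the mouse; otherwise it clears facing.
; The attack executes the ShockBurst cue on authority and plays the montage, whose gameplay event triggers the beam spawn.
; A failed commit cancels the ability.
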(event `self.K2_ActivateAbility`
  (bind _returnvalue (`self.K2_CommitAbility`))
  (if _returnvalue
    (`|ExecutionSequence`
      (:`then_0`
        (bind (_asynctaskproxy _timeheld) (`AbilityTask_WaitInputRelease.WaitInputRelease` true)
          (:`OnRelease`
            (`self.OnInputRelease` _timeheld))))
      (:`then_1`
        (if (`self.ShouldSetMotionTarget`)
          (bind (_asynctaskproxy_2 _datahandle) (`TargetDataUnderMouse.CreateTargetDataUnderMouse`)
            (:`HasMouseTarget`
              (`self.FaceHitTarget` (`AbilitySystemBlueprintLibrary.GetHitResultFromTargetData` _datahandle)))
            (:`HasNoTarget`
              (message `CombatInterface.ClearFacingTarget` (`self.GetAvatarActorFromActorInfo`) :!label _label)))
          (else
            (goto _label)))
        (`self.Execute Attack`)))
    (else
      (`self.K2_CancelAbility`))))

(event `self.PlayAbilitySoundCue`
  (`self.K2_HasAuthority`
    (:`True`
      (`self.K2_ExecuteGameplayCue` (struct :`TagName` "GameplayCue.ShockBurst")))))

(event `self.PlayAbilityMontage`
  (`AbilityTask_PlayMontageAndWait.CreatePlayMontageAndWaitProxy` "None" "/Game/MetaHumans/MHC_Egyptian/Animations/Combat/AM_Egyptian_Attack_Primary.AM_Egyptian_Attack_Primary"
    (:`then`
      (`AbilityTask_WaitGameplayEvent.WaitGameplayEvent` (struct :`TagName` "Event.Montage.Egyptian.Primary") null true
        (:`EventReceived`
          (`self.SpawnBeam`))))))

(event `Execute Attack`
  (`self.PlayAbilitySoundCue`)
  (`self.PlayAbilityMontage`))