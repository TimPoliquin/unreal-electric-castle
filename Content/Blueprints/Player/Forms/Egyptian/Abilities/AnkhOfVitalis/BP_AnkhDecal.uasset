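; BP_AnkhDecal is a glowing decal actor with particles for the Egyptian form's Ankh of Vitalis ability.
; On BeginPlay it starts lit or dark based on StartVisible.
; FadeIn and FadeOut toggle the particles and use timelines to scale the decal's emissive strength, with FadeOut optionally destroying the actor when finished.
; A helper lazily caches the decal's dynamic material instance, creating one if needed.
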(event `self.ReceiveBeginPlay`
  (`self.GetOrCreateDecalDynamicMaterial`)
  (if (`self.Start Visible`)
    (`MaterialInstanceDynamic.SetScalarParameterValue` (`self.Decal Dynamic Material`) "Emissive Strength" (`self.Emmisive Strength`))
    (`ActorComponent.Activate` (`self.Particles`) false)
    (else
      (`MaterialInstanceDynamic.SetScalarParameterValue` (`self.Decal Dynamic Material`) "Emissive Strength" 0.0))))

(event `Fade In`
  (`ActorComponent.Activate` (`self.Particles`) false)
  (`self.GetOrCreateDecalDynamicMaterial`)
  (bind (_direction _alpha) (`Timeline|Fade In Timeline` :!via `PlayFromStart`)
    (:`Update`
      (`MaterialInstanceDynamic.SetScalarParameterValue` (`self.Decal Dynamic Material`) (`self.Emissive Strength Property Name`) (* _alpha (`self.Emmisive Strength`))))
    (:`Finished`
      (`MaterialInstanceDynamic.SetScalarParameterValue` (`self.Decal Dynamic Material`) (`self.Emissive Strength Property Name`) (`self.Emmisive Strength`)))))

(event `Fade Out`
  (params (`Destroy On Finish` :type Boolean))
  (`ActorComponent.Deactivate` (`self.Particles`))
  (`self.GetOrCreateDecalDynamicMaterial`)
  (bind (_direction _alpha) (`Timeline|Fade Out Timeline` :!via `PlayFromStart`)
    (:`Update`
      (`MaterialInstanceDynamic.SetScalarParameterValue` (`self.Decal Dynamic Material`) (`self.Emissive Strength Property Name`) (* _alpha (`self.Emmisive Strength`))))
    (:`Finished`
      (`MaterialInstanceDynamic.SetScalarParameterValue` (`self.Decal Dynamic Material`) (`self.Emissive Strength Property Name`) 0.0)
      (if `Destroy On Finish`
        (`self.K2_DestroyActor`)))))

(fn `GetOrCreateDecalDynamicMaterial`
  (returns (`Decal Material` :type "MaterialInstanceDynamic Object Reference"))
  (`self.Decal Dynamic Material`
    (:`then`
      _)
    (:`else`
      (bind _asmaterial_instance_dynamic (cast `MaterialInstanceDynamic` (`DecalComponent.GetDecalMaterial` (`self.Decal`)))
        (:`then`
          (set `self.Decal Dynamic Material` _asmaterial_instance_dynamic))
        (:`CastFailed`
          (bind _returnvalue (`DecalComponent.CreateDynamicMaterialInstance` (`self.Decal`)))
          (set `self.Decal Dynamic Material` _returnvalue)))))
  (return (`self.Decal Dynamic Material`)))

(fn `UserConstructionScript`)