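; Egyptian form's Ankh of Vitalis secondary ability, a self-heal timed by gameplay events from the attack montage.
; On the authority, montage events apply the Vitalis effect to the avatar, trigger the heal through DamageTarget on itself, then remove the effect.
; A downward trace places an ankh decal on the ground as the montage starts, and the effect-end event fades it out.
; The ability ends when the montage completes, is interrupted or is cancelled.
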(event `self.K2_OnEndAbility`
  (params (bWasCancelled :type Boolean))
  (set `self.AnkhDecal` null))

(event `self.K2_ActivateAbility`
  (bind _returnvalue (`self.K2_CommitAbility`))
  (if _returnvalue
    (`self.Execute Ability`)
    (else
      (`self.K2_CancelAbility`))))

(event `Execute Ability`
  (`AbilityTask_PlayMontageAndWait.CreatePlayMontageAndWaitProxy` "None" "/Game/MetaHumans/MHC_Egyptian/Animations/Combat/AM_Egyptian_Attack_Secondary.AM_Egyptian_Attack_Secondary" 1.0 "None" false
    (:`then`
      (`self.K2_HasAuthority`
        (:`True`
          (`self.Setup Effect Begin`)
          (`self.Setup Heal Effect`)
          (`self.Setup Effect End`)
          (`self.Project Ankh Decal`))))
    (:`OnCompleted`
      (`self.K2_EndAbility` :!label _label))
    (:`OnInterrupted`
      (goto _label))
    (:`OnCancelled`
      (goto _label))))

(event `Setup Effect Begin`
  (`AbilityTask_WaitGameplayEvent.WaitGameplayEvent` (struct :`TagName` "Event.Montage.Egyptian.Secondary.EffectBegin") null
    (:`EventReceived`
      (bind _returnvalue (`ElectricCastleAbilitySystemLibrary.ApplyBasicGameplayEffect` (`self.GetAvatarActorFromActorInfo`) "/Game/Blueprints/Player/Forms/Egyptian/Abilities/AnkhOfVitalis/GE_Egyptian_AnkhOfVitalis.GE_Egyptian_AnkhOfVitalis_C" (`self.GetAbilityLevel`)))
      (set `self.Effect Handle` _returnvalue))))

(event `Setup Heal Effect`
  (bind _returnvalue (`self.GetAvatarActorFromActorInfo`))
  (`AbilityTask_WaitGameplayEvent.WaitGameplayEvent` (struct :`TagName` "Event.Montage.Egyptian.Secondary.Heal") null
    (:`EventReceived`
      (`self.DamageTarget` _returnvalue (`Actor.K2_GetActorLocation` _returnvalue) (`BlueprintGameplayTagLibrary.MakeLiteralGameplayTag` (struct))))))

(event `Setup Effect End`
  (`AbilityTask_WaitGameplayEvent.WaitGameplayEvent` (struct :`TagName` "Event.Montage.Egyptian.Secondary.EffectEnd") null
    (:`EventReceived`
      (`self.Destroy Ankh Decal`)
      (`ElectricCastleAbilitySystemLibrary.RemoveGameplayEffect` (`self.GetAvatarActorFromActorInfo`) (`self.Effect Handle`) false))))

(event `Project Ankh Decal`
  (bind _returnvalue (`Actor.K2_GetActorLocation` (`self.GetAvatarActorFromActorInfo`)))
  (bind (_outhit _returnvalue_2) (`KismetSystemLibrary.LineTraceSingleForObjects` _returnvalue (+ _returnvalue (0.0 0.0 -10000.0)) (`|MakeArray` "ObjectTypeQuery1" "ObjectTypeQuery2" :!type "EObjectTypeQuery Enum") false (`|MakeArray` (`self.GetAvatarActorFromActorInfo`))))
  (if _returnvalue_2
    (bind _returnvalue_3 (`|SpawnActorFromClass` "/Game/Blueprints/Player/Forms/Egyptian/Abilities/AnkhOfVitalis/BP_AnkhDecal.BP_AnkhDecal_C" (`KismetMathLibrary.MakeTransform` (`.Location` (`GameplayStatics.BreakHitResult` _outhit)) (struct :`Pitch` 90.0)) "AlwaysSpawn" "MultiplyWithRoot" null false 15.0 "Emissive Strength" null))
    (bind _output_get (set `self.AnkhDecal` _returnvalue_3))
    (`/Game/Blueprints/Player/Forms/Egyptian/Abilities/AnkhOfVitalis/BP_AnkhDecal.Fade In` _output_get)
    (else
      (`KismetSystemLibrary.PrintString` "Nothing below!"))))

(event `Destroy Ankh Decal`
  (bind _ankhdecal (`self.AnkhDecal`)
    (:`then`
      (`/Game/Blueprints/Player/Forms/Egyptian/Abilities/AnkhOfVitalis/BP_AnkhDecal.Fade Out` _ankhdecal true))
    (:`else`
      (`KismetSystemLibrary.PrintString` "No Ankh"))))