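; Knight Magic Hand gameplay ability that launches a hand projectile and tethers the Knight to whatever it possesses.
; A cast montage event makes the server spawn BP_MagicHand at the attach socket with a cast effect.
; On possess, it plays the movement montage, attaches the tether server-side and swaps to the attached effect.
; A miss or second input press ends the ability, which detaches the tether, removes effects and destroys the hand.
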(event `self.K2_ActivateAbility`
  (bind _returnvalue (`self.K2_CommitAbility`))
  (if _returnvalue
    (`|ExecutionSequence`
      (:`then_0`
        (`self.Cast Hand`))
      (:`then_1`
        (`AbilityTask_WaitInputPress.WaitInputPress` false
          (:`OnPress`
            (`self.Retract Hand`)))))))

(event `Cast Hand`
  (`AbilityTask_PlayMontageAndWait.CreatePlayMontageAndWaitProxy` "None" "/Game/MetaHumans/MHC_Knight/Animation/Abilities/AM_Knight_MagicHand.AM_Knight_MagicHand" 1.0 "Start"
    (:`then`
      (`AbilityTask_WaitGameplayEvent.WaitGameplayEvent` (struct :`TagName` "Event.Montage.Knight.MagicHand") null
        (:`EventReceived`
          (`self.K2_HasAuthority`
            (:`True`
              (`self.Apply Hand of Merlin Cast Effect`)
              (bind _returnvalue (`self.Spawn Hand of Merlin`))
              (`/Engine/EditorBlueprintResources/StandardMacros.IsValid` _returnvalue
                (:`Is Valid`
                  (`|ExecutionSequence`
                    (:`then_0`
                      (set `self.Hand of Merlin` _returnvalue)
                      (`MagicHand.Launch` (`self.Hand of Merlin`) (`self.GetAvatarActorFromActorInfo`) 500.0 (`AbilitySystemBlueprintLibrary.Conv_ScalableFloatToDouble` (`self.Range`) (`KismetMathLibrary.Conv_IntToDouble` (`self.GetAbilityLevel`)))))
                    (:`then_1`
                      (add `MagicHand.OnPossess` (`self.Hand of Merlin`) (delegate `OnPossess_Event`)))
                    (:`then_2`
                      (add `MagicHand.OnMiss` (`self.Hand of Merlin`) (delegate `OnMiss_Event`)))))
                (:`Is Not Valid`
                  (`self.K2_EndAbility`))))))))))

(event `self.K2_OnEndAbility`
  (params (bWasCancelled :type Boolean))
  (bind _returnvalue (message `TetherAbilityActorInterface.GetTetherAbilityComponent` (`self.GetAvatarActorFromActorInfo`)))
  (`TetherAbilityComponent.DetachTarget` _returnvalue)
  (`self.Remove Hand of Merlin Cast Effect`)
  (`self.Remove Hand of Merlin Attached Effect`)
  (`self.Destroy Hand of Merlin`))

(event `OnPossess_Event`
  (params (Payload :type "MagicHandPossessPayload Structure (by ref)"))
  (`self.Handle Hand Hit` Payload))

(event `Retract Hand`
  (`self.K2_EndAbility`))

(event `OnMiss_Event`
  (`self.Handle Hand Miss`))

(event `Handle Hand Hit`
  (params (`Possess Payload` :type "MagicHandPossessPayload Structure"))
  (`self.MontageStop` -1.0)
  (`AbilityTask_PlayMontageAndWait.CreatePlayMontageAndWaitProxy` "None" "/Game/MetaHumans/MHC_Knight/Animation/Abilities/AM_Knight_MagicHand_Movement.AM_Knight_MagicHand_Movement"
    (:`then`
      (`self.K2_HasAuthority`
        (:`True`
          (bind _returnvalue (message `TetherAbilityActorInterface.GetTetherAbilityComponent` (`self.GetAvatarActorFromActorInfo`)))
          (`TetherAbilityComponent.AttachTarget` _returnvalue (`.PossessedActor` (break `MagicHandPossessPayload` `Possess Payload`)))
          (`self.Remove Hand of Merlin Cast Effect`)
          (`self.Apply Hand of Merlin Attached Effect`))))))

(event `Handle Hand Miss`
  (`self.K2_HasAuthority`
    (:`True`
      (`self.K2_EndAbility`))))

(fn `Apply Hand of Merlin Attached Effect`
  (bind _returnvalue (`ElectricCastleAbilitySystemLibrary.ApplyBasicGameplayEffect` (`self.GetAvatarActorFromActorInfo`) "/Game/Blueprints/Player/Forms/Knight/Abilities/MagicHand/GE_MagicHand_Attached.GE_MagicHand_Attached_C"))
  (set `self.Hand of Merlin Attached Effect Handle` _returnvalue))

(fn `Apply Hand of Merlin Cast Effect`
  (bind _returnvalue (`ElectricCastleAbilitySystemLibrary.ApplyBasicGameplayEffect` (`self.GetAvatarActorFromActorInfo`) "/Game/Blueprints/Player/Forms/Knight/Abilities/MagicHand/GE_MagicHand_Cast.GE_MagicHand_Cast_C"))
  (set `self.Hand of Merlin Cast Effect Handle` _returnvalue))

(fn `Destroy Hand of Merlin`
  (bind _hand_of_merlin (`self.Hand of Merlin`)
    (:`then`
      (`Actor.K2_DestroyActor` _hand_of_merlin))
    (:`else`
      _))
  (set `self.Hand of Merlin` null))

(fn `Remove Hand of Merlin Attached Effect`
  (`ElectricCastleAbilitySystemLibrary.RemoveGameplayEffect` (`self.GetAvatarActorFromActorInfo`) (`self.Hand of Merlin Attached Effect Handle`)))

(fn `Remove Hand of Merlin Cast Effect`
  (`ElectricCastleAbilitySystemLibrary.RemoveGameplayEffect` (`self.GetAvatarActorFromActorInfo`) (`self.Hand of Merlin Cast Effect Handle`)))

(fn `Spawn Hand of Merlin`
  (returns (ReturnValue :type "/Game/Blueprints/Player/Forms/Knight/Abilities/MagicHand/BP_MagicHand Object Reference"))
  (bind _returnvalue (`self.GetAvatarActorFromActorInfo`))
  (bind (_attachbonename _returnvalue_2) (message `MagicHandPossessorInterface.GetMagicHandAttachComponent` _returnvalue))
  (`/Engine/EditorBlueprintResources/StandardMacros.IsValid` _returnvalue_2
    (:`Is Valid`
      (bind _returnvalue_3 (`|SpawnActorFromClass` "/Game/Blueprints/Player/Forms/Knight/Abilities/MagicHand/BP_MagicHand.BP_MagicHand_C" (`KismetMathLibrary.MakeTransform` (`SceneComponent.GetSocketLocation` _returnvalue_2 _attachbonename) (`Actor.K2_GetActorRotation` _returnvalue)) "Undefined" "MultiplyWithRoot" (`self.GetAvatarActorFromActorInfo`) (cast `Pawn` (`self.GetAvatarActorFromActorInfo`) :!pure true)))
      (return _returnvalue_3))))