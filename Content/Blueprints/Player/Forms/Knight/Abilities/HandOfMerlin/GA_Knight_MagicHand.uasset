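; Knight gameplay ability that casts the Hand of Merlin, a magic hand that attaches to the target it hits.
; On activation, the server applies a cast effect and spawns BP_MagicHand on the avatar with level-scaled range.
; A hit callback attaches the hand and swaps the cast effect for an attached effect.
; A miss or another input press ends the ability, which removes both effects and destroys the hand.
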(event `self.K2_ActivateAbility`
  (bind _returnvalue (`self.K2_CommitAbility`))
  (if _returnvalue
    (`|ExecutionSequence`
      (:`then_0`
        (`self.Cast Hand`))
      (:`then_1`
        (`AbilityTask_WaitInputPress.WaitInputPress` false
          (:`OnPress`
            (`self.Retract Hand`)))))))

(event `Cast Hand`
  (`self.K2_HasAuthority`
    (:`True`
      (`self.Apply Hand of Merlin Cast Effect`)
      (bind _returnvalue (`self.Spawn Hand of Merlin`))
      (`/Engine/EditorBlueprintResources/StandardMacros.IsValid` _returnvalue
        (:`Is Valid`
          (`|ExecutionSequence`
            (:`then_0`
              (set `self.Hand of Merlin` _returnvalue)
              (`/Game/Blueprints/Player/Forms/Knight/Abilities/HandOfMerlin/BP_MagicHand.Cast` (`self.Hand of Merlin`)))
            (:`then_1`
              (add `/Game/Blueprints/Player/Forms/Knight/Abilities/HandOfMerlin/BP_MagicHand.Hit` (`self.Hand of Merlin`) (delegate `On Hand Hit`)))
            (:`then_2`
              (add `/Game/Blueprints/Player/Forms/Knight/Abilities/HandOfMerlin/BP_MagicHand.No Hit` (`self.Hand of Merlin`) (delegate `On Hand Miss`)))))
        (:`Is Not Valid`
          (`self.K2_EndAbility`))))))

(event `self.K2_OnEndAbility`
  (params (bWasCancelled :type Boolean))
  (`self.Remove Hand of Merlin Cast Effect`)
  (`self.Remove Hand of Merlin Attached Effect`)
  (`self.Destroy Hand of Merlin`))

(event `On Hand Hit`
  (params (Target :type "Actor Object Reference"))
  (`self.Handle Hand Hit` Target))

(event `On Hand Miss`
  (`self.Handle Hand Miss`))

(event `Retract Hand`
  (`self.K2_EndAbility`))

(event `Handle Hand Hit`
  (params (Target :type "Actor Object Reference"))
  (`/Game/Blueprints/Player/Forms/Knight/Abilities/HandOfMerlin/BP_MagicHand.Attach` (`self.Hand of Merlin`) Target)
  (`self.Remove Hand of Merlin Cast Effect`)
  (`self.Apply Hand of Merlin Attached Effect`))

(event `Handle Hand Miss`
  (`self.K2_EndAbility`))

(fn `Apply Hand of Merlin Attached Effect`
  (bind _returnvalue (`ElectricCastleAbilitySystemLibrary.ApplyBasicGameplayEffect` (`self.GetAvatarActorFromActorInfo`) "/Game/Blueprints/Player/Forms/Knight/Abilities/HandOfMerlin/GE_MagicHand_Attached.GE_MagicHand_Attached_C"))
  (set `self.Hand of Merlin Attached Effect Handle` _returnvalue))

(fn `Apply Hand of Merlin Cast Effect`
  (bind _returnvalue (`ElectricCastleAbilitySystemLibrary.ApplyBasicGameplayEffect` (`self.GetAvatarActorFromActorInfo`) "/Game/Blueprints/Player/Forms/Knight/Abilities/HandOfMerlin/GE_MagicHand_Cast.GE_MagicHand_Cast_C"))
  (set `self.Hand of Merlin Cast Effect Handle` _returnvalue))

(fn `Destroy Hand of Merlin`
  (bind _hand_of_merlin (`self.Hand of Merlin`)
    (:`then`
      (`Actor.K2_DestroyActor` _hand_of_merlin))
    (:`else`)))

(fn `Remove Hand of Merlin Attached Effect`
  (`ElectricCastleAbilitySystemLibrary.RemoveGameplayEffect` (`self.GetAvatarActorFromActorInfo`) (`self.Hand of Merlin Attached Effect Handle`)))

(fn `Remove Hand of Merlin Cast Effect`
  (`ElectricCastleAbilitySystemLibrary.RemoveGameplayEffect` (`self.GetAvatarActorFromActorInfo`) (`self.Hand of Merlin Cast Effect Handle`)))

(fn `Spawn Hand of Merlin`
  (returns (ReturnValue :type "/Game/Blueprints/Player/Forms/Knight/Abilities/HandOfMerlin/BP_MagicHand Object Reference"))
  (locals (`Local Hand` :type "/Game/Blueprints/Player/Forms/Knight/Abilities/HandOfMerlin/BP_MagicHand Object Reference"))
  (bind _returnvalue (`self.GetAvatarActorFromActorInfo`))
  (bind _returnvalue_2 (`|SpawnActorFromClass` "/Game/Blueprints/Player/Forms/Knight/Abilities/HandOfMerlin/BP_MagicHand.BP_MagicHand_C" (`Actor.GetTransform` (`self.GetAvatarActorFromActorInfo`)) "Undefined" "MultiplyWithRoot" _returnvalue _returnvalue (`AbilitySystemBlueprintLibrary.Conv_ScalableFloatToDouble` (`self.Range`) (`KismetMathLibrary.Conv_IntToDouble` (`self.GetAbilityLevel`))) (cast `Pawn` (`self.GetAvatarActorFromActorInfo`) :!pure true)))
  (bind _output_get (set `local.Local Hand` _returnvalue_2))
  (`/Game/Blueprints/Player/Forms/Knight/Abilities/HandOfMerlin/BP_MagicHand.Attach to Parent` _output_get)
  (return (`local.Local Hand`)))