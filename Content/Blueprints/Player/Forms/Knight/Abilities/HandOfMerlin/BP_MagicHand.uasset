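; Magic hand projectile for the Knight's Hand of Merlin ability, fired forward to grab an actor.
; Cast launches it via ProjectileMovement and draws a debug sphere at maximum range; overlapping a non-possessor stops it and calls Hit.
; Attach passes the target to the possessor's tether component and snaps the hand onto it.
; Tick is empty, leaving the manual lerp, NoHit timeout and target re-alignment logic disconnected.
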(event `self.ReceiveTick`
  (params (DeltaSeconds :type "Float (single-precision)")))

(event `Attach to Parent`)

(event `Cast`
  (bind _output_get (set `self.Cast Destination` (`self.Calculate Cast Destination`)))
  (`KismetSystemLibrary.DrawDebugSphere` _output_get 25.0 12 (struct :`G` 1.0 :`A` 1.0) 1.0 1.0)
  (set `self.Cast Progress` 0.0)
  (`self.Activate Hand Projectile`)
  (set `self.ShouldCast` true))

(event `Update Cast Progress`
  (params (`Delta Time` :type "Float (double-precision)"))
  (if (< (`self.Cast Progress`) 1.0)
    (bind _returnvalue (`self.Calculate New Cast Progress` `Delta Time`))
    (set `self.Cast Progress` _returnvalue)
    (`SceneComponent.K2_SetWorldLocation` (`self.Hand Mesh`) (`self.Calculate New Cast Position`) false false)
    (else
      (set `self.Cast Progress` 1.0)
      (set `self.ShouldCast` false)
      (`self.No Hit`))))

(event `self.Grab Collision.OnComponentBeginOverlap`
  (params (OverlappedComponent :type "PrimitiveComponent Object Reference") (OtherActor :type "Actor Object Reference") (OtherComp :type "PrimitiveComponent Object Reference") (OtherBodyIndex :type Integer) (bFromSweep :type Boolean) (SweepResult :type "HitResult Structure (by ref)"))
  (if (and (!= OtherActor (`self.Possessor`)) (`self.ShouldCast`))
    (set `self.ShouldCast` false)
    (`MovementComponent.StopMovementImmediately` (`self.ProjectileMovement`))
    (`self.Hit` OtherActor)
    (`ActorComponent.Deactivate` (`self.Grab Collision`))))

(event `Attach`
  (params (`In Target` :type "Actor Object Reference"))
  (set `self.Target` `In Target`)
  (`self.Attach Actor`))

(event `Update Hand Target Position`
  (`/Engine/EditorBlueprintResources/StandardMacros.IsValid` (`self.Target`)
    (:`Is Valid`
      (if (!= (`SceneComponent.K2_GetComponentLocation` (`self.Hand Mesh`)) (`self.K2_GetActorLocation` (`self.Target`)) :`ErrorTolerance` 0.1)
        ; Remap the hand's position to match the target actor
        (`self.K2_DetachFromActor` (`self.Target`) "KeepWorld" "KeepWorld" "KeepRelative")
        (`SceneComponent.K2_SetWorldLocation` (`self.Hand Mesh`) (`self.K2_GetActorLocation` (`self.Target`)) false false)
        (`self.K2_AttachToComponent` (`self.Target`) (`self.Hand Mesh`) "None" "SnapToTarget" "SnapToTarget" "KeepRelative" true)))))

(fn `Activate Hand Projectile`
  (set `ProjectileMovementComponent.InitialSpeed` (`self.Speed`) (`self.ProjectileMovement`))
  (set `ProjectileMovementComponent.MaxSpeed` (`self.Speed`) (`self.ProjectileMovement`))
  (`ProjectileMovementComponent.SetVelocityInLocalSpace` (`self.ProjectileMovement`) (* (`KismetMathLibrary.Vector_Forward`) (`self.Speed`)))
  (`ActorComponent.Activate` (`self.ProjectileMovement`) false))

(fn `Attach Actor`
  (locals (`Physics Constraint` :type "PhysicsConstraintComponent Object Reference"))
  (`self.Target`
    (:`then`
      (bind _returnvalue (message `TetherAbilityActorInterface.GetTetherAbilityComponent` (`self.Possessor`)))
      (`/Engine/EditorBlueprintResources/StandardMacros.IsValid` _returnvalue
        (:`Is Valid`
          (`TetherAbilityComponent.AttachTarget` _returnvalue (`self.Target`))
          (`self.K2_AttachToComponent` (`Actor.RootComponent` (`self.Target`)) "None" "SnapToTarget" "SnapToTarget" "KeepRelative"))
        (:`Is Not Valid`
          (`KismetSystemLibrary.PrintString` "Could not find tether component"))))
    (:`else`)))

(fn `Calculate Cast Destination`
  (returns (ReturnValue :type "Vector Structure"))
  (return (+ (`self.K2_GetActorLocation`) (* (`self.GetActorForwardVector`) (`self.Range`)))))

(fn `Calculate New Cast Position`
  (returns (ReturnValue :type "Vector Structure"))
  (return (`KismetMathLibrary.VLerp` (`self.K2_GetActorLocation` (`self.Possessor`)) (`self.Cast Destination`) (`self.Cast Progress`))))

(fn `Calculate New Cast Progress`
  (params (A :type "Float (double-precision)"))
  (returns (ReturnValue :type "Float (double-precision)"))
  (return (+ (`self.Cast Progress`) (`KismetMathLibrary.SafeDivide` (* A (`self.Speed`)) (`self.Range`)))))

(fn `UserConstructionScript`)