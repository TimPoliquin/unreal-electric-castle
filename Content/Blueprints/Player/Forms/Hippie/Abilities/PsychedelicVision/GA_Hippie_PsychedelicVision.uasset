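; Gameplay Ability for the Hippie form's Psychedelic Vision, a timed vision effect with a configurable radius.
; After commit, a montage event sets the radius in a material parameter collection, then applies the visual effect and a state shift detection component.
; The server applies the active GameplayEffect and ends the ability after its level-scaled lifetime, while another input press ends it early.
; Ending removes the effect and visuals.
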(event `self.K2_ActivateAbility`
  (bind _returnvalue (`self.K2_CommitAbility`))
  (if _returnvalue
    (`self.Play Montage`)))

(event `Play Montage`
  (`AbilityTask_PlayMontageAndWait.CreatePlayMontageAndWaitProxy` "None" "/Game/MetaHumans/MHC_Hippie/Animations/Ability/AM_Hippie_PsychedelicVision.AM_Hippie_PsychedelicVision"
    (:`then`
      (`AbilityTask_WaitGameplayEvent.WaitGameplayEvent` (struct :`TagName` "Event.Montage.Hippie.PsychedelicVision") null
        (:`EventReceived`
          (`self.Execute`))))))

(event `Execute`
  (`KismetMaterialLibrary.SetScalarParameterValue` (`self.Psychedelic Vision Material Parameters`) "Radius" (`self.GetEffectRadius`))
  (`self.ApplyVisualEffect`)
  (`self.ApplyStateShiftDetectionComponent`)
  (`AbilityTask_WaitInputPress.WaitInputPress` false
    (:`then`
      (`self.K2_HasAuthority`
        (:`True`
          (`|ExecutionSequence`
            (:`then_0`
              (`KismetSystemLibrary.Delay` (`AbilitySystemBlueprintLibrary.Conv_ScalableFloatToFloat` (`self.Ability Lifetime`) (`KismetMathLibrary.Conv_IntToDouble` (`self.GetAbilityLevel`))))
              (`self.K2_EndAbility`))
            (:`then_1`
              (bind _returnvalue (`ElectricCastleAbilitySystemLibrary.ApplyBasicGameplayEffect` (`self.GetAvatarActorFromActorInfo`) "/Game/Blueprints/Player/Forms/Hippie/Abilities/PsychedelicVision/GE_Hippie_Attack_PsychedelicVision_Active.GE_Hippie_Attack_PsychedelicVision_Active_C" (`self.GetAbilityLevel`)))
              (set `self.Psychedelic Vision Effect` _returnvalue))))))
    (:`OnPress`
      (`self.K2_EndAbility`))))

(event `self.K2_OnEndAbility`
  (params (bWasCancelled :type Boolean))
  (`self.BP_RemoveGameplayEffectFromOwnerWithHandle` (`self.Psychedelic Vision Effect`) 1)
  (`self.RemoveVisualEffect`)
  (`parent.K2_OnEndAbility` bWasCancelled))