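; Test player character with Enhanced Input move and look, plus a magic hand ability on Interact.
; Movement input is normalized from controller-based vectors, then filtered through the TetherAbility component's limits before being applied.
; Interact spawns and casts a BP_MagicHand owned by the character, whose bound hit and miss events attach it to the target or destroy it.
; Getters expose the pickup anchor and tether component.
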(event `EnhancedInput|/Game/Blueprints/Input/InputActions/IA_Move`
  (params (ActionValue :type "Vector2D Structure") (ElapsedSeconds :type "Float (double-precision)") (TriggeredSeconds :type "Float (double-precision)") (InputAction :type "InputAction Object Reference" :default "/Game/Blueprints/Input/InputActions/IA_Move.IA_Move"))
  (:`Triggered`
    (`self.DoMove` ActionValue_Y ActionValue_X)))

(event `EnhancedInput|/Game/Blueprints/Input/InputActions/IA_Look`
  (params (ActionValue :type "Vector2D Structure") (ElapsedSeconds :type "Float (double-precision)") (TriggeredSeconds :type "Float (double-precision)") (InputAction :type "InputAction Object Reference" :default "/Game/Blueprints/Input/InputActions/IA_Look.IA_Look"))
  (:`Triggered`
    (`self.DoLook` ActionValue_X ActionValue_Y)))

(event `EnhancedInput|/Game/Blueprints/Input/InputActions/IA_Interact`
  (params (ActionValue :type "Float (double-precision)") (ElapsedSeconds :type "Float (double-precision)") (TriggeredSeconds :type "Float (double-precision)") (InputAction :type "InputAction Object Reference" :default "/Game/Blueprints/Input/InputActions/IA_Interact.IA_Interact"))
  (:`Started`
    (`self.Do Magic Hand`)))

(event `Do Magic Hand`
  (bind _returnvalue (`|SpawnActorFromClass` "/Game/Blueprints/Player/Forms/Knight/Abilities/HandOfMerlin/BP_MagicHand.BP_MagicHand_C" (`self.GetTransform`) "Undefined" "MultiplyWithRoot" self self 200.0 null))
  (add `/Game/Blueprints/Player/Forms/Knight/Abilities/HandOfMerlin/BP_MagicHand.Hit` _returnvalue (delegate `Hit_Event`))
  (add `/Game/Blueprints/Player/Forms/Knight/Abilities/HandOfMerlin/BP_MagicHand.No Hit` _returnvalue (delegate `No Hit_Event`))
  (`/Game/Blueprints/Player/Forms/Knight/Abilities/HandOfMerlin/BP_MagicHand.Cast` _returnvalue))

(event `Hit_Event`
  (params (Target :type "Actor Object Reference"))
  (`self.On Magic Hand Hit` (stale `Do Magic Hand` _returnvalue) Target))

(event `No Hit_Event`
  (`self.On Magic Hand Miss` (stale `Do Magic Hand` _returnvalue)))

(event `On Magic Hand Hit`
  (params (`Magic Hand` :type "/Game/Blueprints/Player/Forms/Knight/Abilities/HandOfMerlin/BP_MagicHand Object Reference") (`In Target` :type "Actor Object Reference"))
  (`/Game/Blueprints/Player/Forms/Knight/Abilities/HandOfMerlin/BP_MagicHand.Attach` `Magic Hand` `In Target`))

(event `On Magic Hand Miss`
  (params (`Magic Hand` :type "Actor Object Reference"))
  (`self.K2_DestroyActor` `Magic Hand`))

(fn `DoLook`
  (params (Yaw :type "Float (double-precision)") (Pitch :type "Float (double-precision)"))
  (`/Engine/EditorBlueprintResources/StandardMacros.IsValid` (`self.GetController`)
    (:`Is Valid`
      (`self.AddControllerYawInput` (`local.Yaw`))
      (`self.AddControllerPitchInput` (`local.Pitch`)))))

(fn `DoMove`
  (params (Forward :type "Float (double-precision)") (Right :type "Float (double-precision)"))
  (locals (`Forward Restricted` :type Boolean :default false) (`Movement Direction` :type "Vector Structure" :default (0.0 0.0 0.0)) (`Right Vector` :type "Vector Structure" :default (0.0 0.0 0.0)))
  (bind (_outdirection _outscale) (`TetherAbilityComponent.ModifyInputMovementByTetherLimits` (`self.TetherAbility`) (`local.Movement Direction`) 1.0))
  (bind (_outforward _outright) (`ElectricCastlePlayerController.GetMovementVectors` (`self.GetController`)))
  (`/Engine/EditorBlueprintResources/StandardMacros.IsValid` (`self.GetController`)
    (:`Is Valid`
      (set `local.Movement Direction` (`KismetMathLibrary.Normal` (+ (* _outforward (`local.Forward`)) (* _outright (`local.Right`)))))
      (`self.AddMovementInput` _outdirection _outscale))))

(fn `Get Magic Hand Attach Component`
  (returns (`Magic Hand Attachment` :type "PrimitiveComponent Object Reference"))
  (return (`self.PickupAnchor`)))

(fn `GetTetherAbilityComponent`
  (returns (ReturnValue :type "TetherAbilityComponent Object Reference"))
  (return (`self.TetherAbility`)))

(fn `UserConstructionScript`)