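; BP_Test_Tether is a test character that travels along a spline and tows a tethered attachment.
; On BeginPlay it takes the spline from its attach parent and binds the attachment's mesh to PickupAnchor through the attachment's physics constraint, with limited X travel and gravity off.
; Tick advances a looping spline distance at max speed and feeds that point's forward direction into movement input.
; It also returns its Mesh as the magic hand attach component.
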(event `self.ReceiveBeginPlay`
  (`self.Find Path`)
  (`self.Attach Actor`))

(event `self.ReceiveTick`
  (params (DeltaSeconds :type "Float (single-precision)"))
  (set `self.DistanceAlongSpline` (mod (+ (`self.DistanceAlongSpline`) (* DeltaSeconds (`MovementComponent.GetMaxSpeed` (`self.CharacterMovement`)))) (`SplineComponent.GetSplineLength` (`self.Travel Path`))))
  (`self.AddMovementInput` (`KismetMathLibrary.GetForwardVector` (`SplineComponent.GetRotationAtDistanceAlongSpline` (`self.Travel Path`) (`self.DistanceAlongSpline`) "Local")) (`MovementComponent.GetMaxSpeed` (`self.CharacterMovement`))))

(fn `Attach Actor`
  (locals (`Physics Constraint` :type "PhysicsConstraintComponent Object Reference"))
  (bind _attachment (`self.Attachment`)
    (:`then`
      (`self.K2_AddActorLocalOffset` _attachment (0.0 0.0 20.0) false false)
      (bind _physics_constraint (message `/Game/Blueprints/Player/Forms/Knight/Abilities/HandOfMerlin/BI_MagicHand_Pickup.Get Physics Constraint` _attachment))
      (bind _output_get (set `local.Physics Constraint` _physics_constraint))
      (bind _returnvalue (`self.GetComponentByClass` _attachment "/Script/Engine.MeshComponent"))
      (`PhysicsConstraintComponent.SetConstrainedComponents` _output_get _returnvalue "None" (`self.PickupAnchor`) "None")
      (`PhysicsConstraintComponent.SetLinearXLimit` (`local.Physics Constraint`) "LCM_Limited" 200.0)
      (`PrimitiveComponent.SetSimulatePhysics` _returnvalue true)
      (`PrimitiveComponent.SetEnableGravity` _returnvalue false))
    (:`else`)))

(fn `Find Path`
  (bind _returnvalue (`self.GetAttachParentActor`))
  (`/Engine/EditorBlueprintResources/StandardMacros.IsValid` _returnvalue
    (:`Is Valid`
      (set `self.Travel Path` (`self.GetComponentByClass` _returnvalue "/Script/Engine.SplineComponent")))))

(fn `Get Magic Hand Attach Component`
  (returns (`Magic Hand Attachment` :type "PrimitiveComponent Object Reference"))
  (return (`self.Mesh`)))

(fn `UserConstructionScript`)