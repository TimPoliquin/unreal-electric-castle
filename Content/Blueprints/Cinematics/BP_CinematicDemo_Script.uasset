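; Scripted cinematic demo actor that plays a barbarian encounter with a kill-or-leave player choice.
; A trigger plays the intro sequence with override music, then loops a second sequence while a dialog wheel awaits input.
; The choice, or a time-up event defaulting to leave, plays the matching outcome sequence.
; The ending restores the player and music, solves the puzzle, and destroys itself and listed actors.
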(event `Play Background Music`
  (if (`self.Play BGM`)
    (`MusicManagerSubsystem.StartOverrideMusic` (subsystem `MusicManagerSubsystem`) (`self.BGM`) -1.0 -1.0)))

(event `TriggerInterface.OnTrigger`
  (params (InActivate :type Boolean))
  (`AsyncPlayLevelSequence.AsyncPlayLevelSequence` "/Game/Blueprints/Cinematics/Playground/Shots/SH_Basic_001.SH_Basic_001" (make `MovieSceneSequencePlaybackSettings` false (struct) (struct :`bAllowRounding` true) 1.0 0.0 false true true true true false "ForceKeepState" true)
    (:`then`
      (`self.SetActorHiddenInGame` (`GameplayStatics.GetPlayerPawn` 0) true)
      (`self.Play Background Music`))
    (:`OnFinished`
      (`self.Play Decision Loop`))))

(event `Play Decision Loop`
  (bind _payload (`AsyncPlayLevelSequence.AsyncPlayLevelSequence` "/Game/Blueprints/Cinematics/Playground/Shots/SH_Basic_002_Loop.SH_Basic_002_Loop" (make `MovieSceneSequencePlaybackSettings` false (make `MovieSceneSequenceLoopCount` -1) (struct :`bAllowRounding` true) 1.0 0.0 false true true true true false "ForceKeepState" true))
    (:`OnPlay`
      (`self.On Barbarian Decision Available` (`.SequencePlayer` (break `LevelSequenceEventPayload` _payload))))))

(event `On Barbarian Decision Available`
  (params (`Current Sequence` :type "LevelSequencePlayer Object Reference"))
  (set `self.Decide` true)
  (bind _outputpin (`self.Create Dialog Widget`))
  (add `DialogWheelWidget.OnDialogChoiceConfirmed` _outputpin (delegate `OnDialogChoiceConfirmed_Event`)))

(event `OnDialogChoiceConfirmed_Event`
  (params (Payload :type "DialogChoiceConfirmedPayload Structure (by ref)"))
  (`MovieSceneSequencePlayer.Stop` (stale `On Barbarian Decision Available` `Current Sequence`))
  (set `self.Decide` false)
  (`|SwitchGameplayTag` Payload_SelectionTag
    (:`InputTag.Dialog.Left`
      (`self.Play Leave Decision`))
    (:`InputTag.Dialog.Right`
      (`self.Play Kill Decision`))))

(event `On Barbarian Decision Time Up`
  (if (`self.Decide`)
    (set `self.Decide` false)
    (`Widget.RemoveFromParent` (`self.Dialog Wheel Widget`))
    (`self.Play Leave Decision`)))

(event `End`
  (`self.SetActorHiddenInGame` (`GameplayStatics.GetPlayerPawn` 0) false)
  (`self.Destroy Dialog Widget`)
  (`self.K2_DestroyActor`)
  (`/Game/Blueprints/LevelAssets/Test/BP_PuzzleManager_Base.Solve` (`self.Puzzle Manager`))
  (`MusicManagerSubsystem.EndOverrideMusic` (subsystem `MusicManagerSubsystem`) -1.0 -1.0)
  (for _array_element (`self.Destroy On End`)
    (`self.K2_DestroyActor` _array_element)))

(event `Play Kill Decision`
  (`self.Destroy Dialog Widget`)
  (`AsyncPlayLevelSequence.AsyncPlayLevelSequence` "/Game/Blueprints/Cinematics/Playground/Shots/SH_Basic_003_Kill.SH_Basic_003_Kill" (make `MovieSceneSequencePlaybackSettings` false (struct) (struct :`bAllowRounding` true) 1.0 0.0 false false false true true)
    (:`OnFinished`
      (`self.End`))))

(event `Play Leave Decision`
  (`self.Destroy Dialog Widget`)
  (`AsyncPlayLevelSequence.AsyncPlayLevelSequence` "/Game/Blueprints/Cinematics/Playground/Shots/SH_Basic_003_Leave.SH_Basic_003_Leave" (make `MovieSceneSequencePlaybackSettings` false (struct) (struct :`bAllowRounding` true) 1.0 0.0 false false false true true)
    (:`OnFinished`
      (`self.End`))))

(event `Shake Camera`
  (`GameplayStatics.PlayWorldCameraShake` "/Game/FAB/Vefects/Zap_VFX/Shared/Cam/Cam_Shake.Cam_Shake_C"))

(fn `Create Dialog Widget`
  (returns (OutputPin :type "/Game/Blueprints/UI/Dialog/WBP_DialogWheel Object Reference"))
  (bind (_returnvalue_x _returnvalue_y) (`KismetMathLibrary.BreakVector2D` (`WidgetLayoutLibrary.GetViewportSize`)))
  (bind _returnvalue (`|CreateWidget` "/Game/Blueprints/UI/Dialog/WBP_DialogWheel.WBP_DialogWheel_C" (`GameplayStatics.GetPlayerController` 0)))
  (bind _output_get (set `self.Dialog Wheel Widget` _returnvalue))
  (`DialogWheelWidget.AddDialogChoice` _output_get (make `DialogChoice` (struct :`TagName` "InputTag.Dialog.Left") "Leave it Alone"))
  (`DialogWheelWidget.AddDialogChoice` _output_get (make `DialogChoice` (struct :`TagName` "InputTag.Dialog.Right") "Kill it"))
  (`UserWidget.AddToViewport` _output_get 0)
  (`/Game/Blueprints/UI/Dialog/WBP_DialogWheel.Show` _output_get true)
  (`UserWidget.SetPositionInViewport` _output_get (`KismetMathLibrary.MakeVector2D` (- (/ _returnvalue_x 2.0) 196.0) (- _returnvalue_y 256.0)) true)
  (return _output_get))

(fn `Destroy Dialog Widget`
  (bind _dialog_wheel_widget (`self.Dialog Wheel Widget`))
  (`/Engine/EditorBlueprintResources/StandardMacros.IsValid` _dialog_wheel_widget
    (:`Is Valid`
      (`DialogWheelWidget.Hide` _dialog_wheel_widget true)
      (`Widget.RemoveFromParent` _dialog_wheel_widget))))

(fn `UserConstructionScript`)