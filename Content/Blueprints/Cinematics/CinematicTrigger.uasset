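; Cinematic trigger actor that plays an assigned Level Sequence when its OnTrigger event fires with Activate set.
; On activation it creates a sequence player, hides player 0's pawn and starts playback.
; A bound OnFinished callback destroys the spawned sequence actor and shows the pawn again.
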(event `/Game/Blueprints/LevelAssets/Button/BI_Triggerable.OnTrigger`
  (params (Activate :type Boolean))
  (if Activate
    (bind (_outactor _returnvalue) (`LevelSequencePlayer.CreateLevelSequencePlayer` (`self.Level Sequence`)))
    (set `self.Level Sequence Actor` _outactor)
    (bind _output_get (set `self.Level Sequence Player` _returnvalue))
    (add `MovieSceneSequencePlayer.OnFinished` _output_get (delegate `OnFinished_Event`))
    (`self.SetActorHiddenInGame` (`GameplayStatics.GetPlayerPawn` 0) true)
    (`MovieSceneSequencePlayer.Play` (`self.Level Sequence Player`))))

(event `OnFinished_Event`
  (`self.K2_DestroyActor` (`self.Level Sequence Actor`))
  (`self.SetActorHiddenInGame` (`GameplayStatics.GetPlayerPawn` 0) false))

(fn `UserConstructionScript`)