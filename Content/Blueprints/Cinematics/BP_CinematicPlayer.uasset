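; Cinematic actor that, on OnTrigger, hides the player pawn and plays a three-part Level Sequence chain with a barbarian decision window.
; Async play nodes chain on Finished, with input, player and HUD suppressed for the intro and loop shots.
; The loop shot opens the decision with its playback end time, but choice and time-up handling only set a flag and print.
; Sequence 003A always follows, then the pawn is unhidden and the actor destroyed.
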(event `TriggerInterface.OnTrigger`
  (params (InActivate :type Boolean))
  (`AsyncPlayLevelSequence.AsyncPlayLevelSequence` "/Game/Blueprints/Cinematics/Playground/Shots/SH_Basic_001.SH_Basic_001" (make `MovieSceneSequencePlaybackSettings` false (struct) (struct :`bAllowRounding` true) 1.0 0.0 false true true true true false "ForceKeepState" true)
    (:`then`
      (`self.SetActorHiddenInGame` (`GameplayStatics.GetPlayerPawn` 0) true))
    (:`OnFinished`
      (bind _payload (`AsyncPlayLevelSequence.AsyncPlayLevelSequence` "/Game/Blueprints/Cinematics/Playground/Shots/SH_Basic_002_Loop.SH_Basic_002_Loop" (make `MovieSceneSequencePlaybackSettings` false (struct) (struct :`bAllowRounding` true) 1.0 0.0 false true true true true false "ForceKeepState" true))
        (:`OnPlay`
          (bind _returnvalue (`MovieSceneSequenceExtensions.GetPlaybackEndSeconds` (`.Sequence` (break `LevelSequenceEventPayload` _payload))))
          (`self.On Barbarian Decision Available` _returnvalue))
        (:`OnFinished`
          (`AsyncPlayLevelSequence.AsyncPlayLevelSequence` "/Game/Blueprints/Cinematics/Playground/Shots/SH_Basic_003A.SH_Basic_003A"
            (:`OnFinished`
              (`self.End`))))))))

(event `On Barbarian Decision Available`
  (params (`Time Remaining` :type "Float (double-precision)"))
  (`KismetSystemLibrary.PrintString` (`KismetStringLibrary.Concat_StrStr` "Time Remaining: " (`KismetStringLibrary.Conv_DoubleToString` `Time Remaining`)))
  (set `self.Decide` true))

(event `On Barbarian Decision Time Up`
  (if (`self.Decide`)
    (set `self.Decide` false)
    (`KismetSystemLibrary.PrintString` "Time's Up!")))

(event `End`
  (`self.SetActorHiddenInGame` (`GameplayStatics.GetPlayerPawn` 0) false)
  (`self.K2_DestroyActor`))

(fn `UserConstructionScript`)