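; Hippie gameplay ability that activates Psychedelic Vision, a timed vision mode that can be cancelled with another input press.
; On commit it writes the effect radius to a material parameter collection, then applies the visual effect and a state-shift detection component.
; The authority applies the active gameplay effect and ends the ability after a level-scaled lifetime.
; Ending removes the gameplay effect and visual effect.
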(event `self.K2_ActivateAbility`
  (bind _returnvalue (`self.K2_CommitAbility`))
  (if _returnvalue
    (`KismetMaterialLibrary.SetScalarParameterValue` (`self.Psychedelic Vision Material Parameters`) "Radius" (`self.GetEffectRadius`))
    (`self.ApplyVisualEffect`)
    (`self.ApplyStateShiftDetectionComponent`)
    (`AbilityTask_WaitInputPress.WaitInputPress` false
      (:`then`
        (`self.K2_HasAuthority`
          (:`True`
            (`|ExecutionSequence`
              (:`then_0`
                (`KismetSystemLibrary.Delay` (`AbilitySystemBlueprintLibrary.Conv_ScalableFloatToFloat` (`self.Ability Lifetime`) (`KismetMathLibrary.Conv_IntToDouble` (`self.GetAbilityLevel`))))
                (`self.K2_EndAbility`))
              (:`then_1`
                (bind _returnvalue_2 (`ElectricCastleAbilitySystemLibrary.ApplyBasicGameplayEffect` (`self.GetAvatarActorFromActorInfo`) "/Game/Blueprints/AbilitySystem/Ability/Hippie/PsychedelicVision/GE_Hippie_Attack_PsychedelicVision_Active.GE_Hippie_Attack_PsychedelicVision_Active_C" (`self.GetAbilityLevel`)))
                (set `self.Psychedelic Vision Effect` _returnvalue_2))))))
      (:`OnPress`
        (`self.K2_EndAbility`)))))

(event `self.K2_OnEndAbility`
  (params (bWasCancelled :type Boolean))
  (`self.BP_RemoveGameplayEffectFromOwnerWithHandle` (`self.Psychedelic Vision Effect`) 1)
  (`self.RemoveVisualEffect`)
  (`parent.K2_OnEndAbility` bWasCancelled))