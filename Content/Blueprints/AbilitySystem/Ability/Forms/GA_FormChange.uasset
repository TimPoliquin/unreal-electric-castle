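; GA_FormChange is an event-triggered Gameplay Ability that switches the avatar to the form named by the event tag.
; It gets the avatar's form change component through a message call and proceeds only if that component is valid and its current form tag differs exactly.
; On success it starts an asynchronous form change, then commits and ends without waiting; otherwise it just ends.
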(event `self.K2_ActivateAbilityFromEvent`
  (params (EventData :type "GameplayEventData Structure (by ref)"))
  (bind (_can_change_forms _form_change_component) (`self.CanChangeForms` EventData_EventTag))
  (if _can_change_forms
    (`PlayerFormChangeComponent.ChangeForm_Async` _form_change_component EventData_EventTag)
    (`self.K2_CommitAbility`)
    (`self.K2_EndAbility`)
    (else
      (`self.K2_EndAbility`))))

(fn `CanChangeForms`
  (params (`New Form Tag` :type "GameplayTag Structure"))
  (returns (`Can Change Forms` :type Boolean) (`Form Change Component` :type "PlayerFormChangeComponent Object Reference"))
  (locals (`Local Form Change Component` :type "PlayerFormChangeComponent Object Reference") (`Local Can Change Forms` :type Boolean))
  (bind _returnvalue (message `FormChangeActorInterface.GetFormChangeComponent` (`self.GetAvatarActorFromActorInfo`)))
  (bind _output_get (set `local.Local Form Change Component` _returnvalue))
  (`/Engine/EditorBlueprintResources/StandardMacros.IsValid` _output_get
    (:`Is Valid`
      (set `local.Local Can Change Forms` (not (`BlueprintGameplayTagLibrary.MatchesTag` (`PlayerFormChangeComponent.GetCurrentFormTag` (`local.Local Form Change Component`)) (`local.New Form Tag`) true))))
    (:`Is Not Valid`
      (set `local.Local Can Change Forms` false)))
  (return (`local.Local Can Change Forms`) (`local.Local Form Change Component`)))