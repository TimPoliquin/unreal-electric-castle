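; Passive gameplay ability that turns gameplay events under the Attributes tag hierarchy into gameplay effects on its owner.
; On activation it waits for those events, builds a spec from EventBasedEffectClass and applies it to its own ability system component.
; Each tag in EventTags becomes a SetByCaller magnitude: the event's magnitude for an exact match, zero otherwise, so one effect class serves every listed tag.
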(event `self.K2_ActivateAbility`
  (bind (_asynctaskproxy _payload) (`AbilityTask_WaitGameplayEvent.WaitGameplayEvent` (struct :`TagName` "Attributes") null false false)
    (:`EventReceived`
      (bind (_eventtag _instigator _target _optionalobject _optionalobject2 _contexthandle _instigatortags _targettags _eventmagnitude) (break `GameplayEventData` _payload))
      (bind _spechandle (`self.SetTagMagnitudes` _eventtag _eventmagnitude (`self.CreateOutgoingSpec`)))
      (`AbilitySystemComponent.BP_ApplyGameplayEffectSpecToSelf` (`self.GetAbilitySystemComponentFromActorInfo`) _spechandle))))

(fn `CreateOutgoingSpec`
  (returns (Spec :type "GameplayEffectSpecHandle Structure"))
  (bind _returnvalue (`self.GetAbilitySystemComponentFromActorInfo`))
  (return (`AbilitySystemComponent.MakeOutgoingSpec` _returnvalue (`self.EventBasedEffectClass`) 1.0 (`AbilitySystemComponent.MakeEffectContext` _returnvalue))))

(fn `SetTagMagnitudes`
  (params (EventTag :type "GameplayTag Structure") (EventMagnitude :type "Float (double-precision)") (Spec :type "GameplayEffectSpecHandle Structure"))
  (returns (SpecHandle :type "GameplayEffectSpecHandle Structure"))
  (for _array_element (`self.EventTags`)
    (if (`BlueprintGameplayTagLibrary.MatchesTag` _array_element (`local.EventTag`) true)
      (`AbilitySystemBlueprintLibrary.AssignTagSetByCallerMagnitude` (`local.Spec`) _array_element (`local.EventMagnitude`))
      (else
        (`AbilitySystemBlueprintLibrary.AssignTagSetByCallerMagnitude` (`local.Spec`) _array_element))))
  (return (`local.Spec`)))