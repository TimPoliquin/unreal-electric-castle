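; Gameplay ability for fishing that starts an interaction with the interactable actor nearest to the avatar.
; On activation it gathers actors by interface, keeps the closest as an InteractionInterface and sends it an interact message with the avatar.
; The ability ends at once if none is valid; otherwise it stays active.
; On end it sends the stored interactable an interaction end message, always flagged as not cancelled.
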(event `self.K2_ActivateAbility`
  (bind _interactable (`self.GetInteractionActor`))
  (set `self.Interactable` _interactable)
  (`/Engine/EditorBlueprintResources/StandardMacros.IsValid` (`KismetSystemLibrary.Conv_InterfaceToObject` _interactable)
    (:`Is Valid`
      (message `InteractionInterface.OnInteract` (`KismetSystemLibrary.Conv_InterfaceToObject` (`self.Interactable`)) (`self.GetAvatarActorFromActorInfo`)))
    (:`Is Not Valid`
      (`self.K2_EndAbility`))))

(event `self.K2_OnEndAbility`
  (params (bWasCancelled :type Boolean))
  (`/Engine/EditorBlueprintResources/StandardMacros.IsValid` (`KismetSystemLibrary.Conv_InterfaceToObject` (`self.Interactable`))
    (:`Is Valid`
      (message `InteractionInterface.OnInteractionEnd` (`KismetSystemLibrary.Conv_InterfaceToObject` (`self.Interactable`)) (`self.GetAvatarActorFromActorInfo`) false))))

(fn `GetInteractionActor`
  (returns (Interactable :type "InteractionInterface Interface"))
  (locals (ClosestInteractableActors :type "Array of Actor Object Reference"))
  (bind _outactors (`GameplayStatics.GetAllActorsWithInterface` null))
  (bind _outactors_2 (`ElectricCastleAbilitySystemLibrary.GetClosestActors` 1 (`Actor.K2_GetActorLocation` (`self.GetAvatarActorFromActorInfo`)) _outactors))
  (bind _output_get (set `local.ClosestInteractableActors` _outactors_2))
  (if (`KismetArrayLibrary.Array_IsNotEmpty` _output_get)
    (bind _asinteraction_interface (cast `InteractionInterface` (`|GetArrayItem` (`local.ClosestInteractableActors`)))))
  (return _asinteraction_interface))