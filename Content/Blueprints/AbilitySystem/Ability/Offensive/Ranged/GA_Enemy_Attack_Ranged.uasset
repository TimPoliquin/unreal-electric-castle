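; GA_Enemy_Attack_Ranged is an enemy gameplay ability that performs a ranged attack on its target.
; On activation it faces the target, plays a random attack montage, and ends when that montage completes, is interrupted or is cancelled.
; Gameplay events drive the timing: the montage's tag fires the projectile once, while a FaceTarget event turns the enemy toward the target again during the attack.
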(event `self.K2_ActivateAbility`
  (`self.FaceTarget`)
  (bind _output_get (set `self.Selected Montage` (`self.GetRandomAttackMontage`)))
  (`AbilityTask_PlayMontageAndWait.CreatePlayMontageAndWaitProxy` "RangedAttack" (break `TaggedMontage` _output_get) 1.0 "None" false
    (:`then`
      (`self.Wait For Fire Event`)
      (`self.Wait for Update Target Position`))
    (:`OnCompleted`
      (`self.K2_EndAbility` :!label _label))
    (:`OnInterrupted`
      (goto _label))
    (:`OnCancelled`
      (goto _label))))

(event `Wait For Fire Event`
  (`AbilityTask_WaitGameplayEvent.WaitGameplayEvent` (`.MontageTag` (break `TaggedMontage` (`self.Selected Montage`))) null true
    (:`EventReceived`
      (`self.FireProjectileAtTarget` (`.MontageTag` (break `TaggedMontage` (`self.Selected Montage`)))))))

(event `Wait for Update Target Position`
  (`AbilityTask_WaitGameplayEvent.WaitGameplayEvent` (struct :`TagName` "Event.Montage.Target.FaceTarget") null
    (:`EventReceived`
      (`self.FaceTarget`))))