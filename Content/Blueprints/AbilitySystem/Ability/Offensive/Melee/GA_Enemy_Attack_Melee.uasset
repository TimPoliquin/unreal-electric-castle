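; Gameplay ability for enemy melee attacks: the enemy faces its target, plays a random attack montage and damages targets at the impact point.
; A gameplay event matching the montage's tag triggers a search for targets within that montage's impact radius, applies damage to them and ends the ability.
; The ability also ends when the montage completes, is interrupted or is cancelled, and the montage is set to keep playing after the ability ends.
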(event `self.K2_ActivateAbility`
  (`self.FaceTarget`)
  (bind _output_get (set `self.Attack Montage` (`self.GetRandomAttackMontage`)))
  (bind (_montage _montagetag) (break `TaggedMontage` _output_get))
  (`AbilityTask_PlayMontageAndWait.CreatePlayMontageAndWaitProxy` "None" _montage 1.0 "None" false
    (:`then`
      (`AbilityTask_WaitGameplayEvent.WaitGameplayEvent` _montagetag null
        (:`EventReceived`
          (bind (_outtargets _returnvalue) (`self.GetTargetsAtImpact` _montagetag (`self.Get Montage Impact Radius`) (`self.bDebug`)))
          (`self.DamageTargets` _outtargets _returnvalue _montagetag)
          (`self.K2_EndAbility`))))
    (:`OnCompleted`
      (`self.K2_EndAbility` :!label _label))
    (:`OnInterrupted`
      (goto _label))
    (:`OnCancelled`
      (goto _label))))

(fn `Get Montage Impact Radius`
  (returns (`Impact Radius` :type "Float (double-precision)"))
  (return (`.ImpactRadius` (break `TaggedMontage` (`self.Attack Montage`)))))