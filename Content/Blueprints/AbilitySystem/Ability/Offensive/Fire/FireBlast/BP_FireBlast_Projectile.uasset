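; Fire Blast ability projectile that flies out to an apex point, returns toward its starting location, then explodes.
; On BeginPlay, the authority drives movement with two chained timelines that lerp actor location without sweeping.
; During the return leg it checks explode distance each update, completing early when in range or when the timeline finishes.
; Completion plays the impact effect, calls Explode and destroys the actor.
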(event `self.ReceiveBeginPlay`
  (`/Engine/EditorBlueprintResources/ActorMacros.Switch Has Authority`
    (:`Authority`
      (bind (_direction _alpha) (`Timeline|Outgoing Timeline` :!via `PlayFromStart`)
        (:`Update`
          (`self.K2_SetActorLocation` (`KismetMathLibrary.VLerp` (`self.InitialLocation`) (`self.ApexLocation`) _alpha)))
        (:`Finished`
          (bind (_direction_2 _alpha_2) (`Timeline|Incoming Timeline` :!via `PlayFromStart`)
            (:`Update`
              (`self.K2_SetActorLocation` (`KismetMathLibrary.VLerp` (`self.ApexLocation`) (`self.InitialLocation`) _alpha_2))
              (if (`self.IsWithinExplodeDistance`)
                (`self.On Complete`)))
            (:`Finished`
              (`self.On Complete`))))))))

(event `On Complete`
  (`/Engine/EditorBlueprintResources/StandardMacros.IsValid` self
    (:`Is Valid`
      (`self.PlayImpactEffect`)
      (`self.Explode`)
      (`self.K2_DestroyActor`))))

(fn `UserConstructionScript`)