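; Fire Bolt projectile actor for an offensive fire ability, built to be reused through object pooling.
; A single Speed variable drives both initial and max speed of the ProjectileMovement component, applied on construction, at BeginPlay and whenever SetProjectileSpeed is called.
; Pool retrieve and return events extend the parent's handling by activating and deactivating the Fireball component.
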(event `self.ReceiveBeginPlay`
  (`self.InitializeSpeed`))

(event `Set Projectile Speed`
  (params (`In Speed` :type "Float (double-precision)"))
  (set `self.Speed` `In Speed`)
  (`self.InitializeSpeed`))

(event `self.OnPool_FinishRetrieve`
  (params (Payload :type "SpawnPoolEventPayload Structure (by ref)"))
  (`parent.OnPool_FinishRetrieve` Payload)
  (`ActorComponent.Activate` (`self.Fireball`) true))

(event `self.OnPool_Returned`
  (params (Payload :type "SpawnPoolEventPayload Structure (by ref)"))
  (`parent.OnPool_Returned` Payload)
  (`ActorComponent.Deactivate` (`self.Fireball`)))

(fn `InitializeSpeed`
  (set `ProjectileMovementComponent.InitialSpeed` (`self.Speed`) (`self.ProjectileMovement`))
  (set `ProjectileMovementComponent.MaxSpeed` (`self.Speed`) (`self.ProjectileMovement`)))

(fn `UserConstructionScript`
  (`self.InitializeSpeed`))