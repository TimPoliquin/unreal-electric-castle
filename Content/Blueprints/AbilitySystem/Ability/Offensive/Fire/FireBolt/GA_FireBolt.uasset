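; GA_FireBolt is the player's offensive Fire Bolt gameplay ability, which casts projectiles toward the point under the mouse.
; On activation it commits, sets the avatar's active ability tag, reads mouse target data and turns the avatar toward the hit point, ending if there is none.
; It plays the cast montage and spawns projectiles at a montage gameplay event, passing the hit actor as target.
; The ability ends with the montage and clears the tag.
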(event `self.K2_ActivateAbility`
  (`self.K2_CommitAbility`)
  (message `CombatInterface.SetActiveAbilityTag` (`self.GetAvatarActorFromActorInfo`) (`BlueprintGameplayTagLibrary.MakeLiteralGameplayTag` (struct :`TagName` "Abilities.Offensive.Fire.FireBolt")))
  (bind (_asynctaskproxy _datahandle) (`TargetDataUnderMouse.CreateTargetDataUnderMouse`)
    (:`HasMouseTarget`
      (bind (_bblockinghit _binitialoverlap _time _distance _location _impactpoint _normal _impactnormal _physmat _hitactor) (`GameplayStatics.BreakHitResult` (`AbilitySystemBlueprintLibrary.GetHitResultFromTargetData` _datahandle)))
      (bind _output_get (set `self.Projectile Target Location` _impactpoint))
      (message `CombatInterface.UpdateFacingTarget` (`self.GetAvatarActorFromActorInfo`) _output_get)
      (`AbilityTask_PlayMontageAndWait.CreatePlayMontageAndWaitProxy` "None" "/Game/Blueprints/Aura/Animations/AM_Player_Cast_FireBolt.AM_Player_Cast_FireBolt" 1.0 "None" false
        (:`then`
          (`AbilityTask_WaitGameplayEvent.WaitGameplayEvent` (struct :`TagName` "Event.Montage.FireBolt") null
            (:`EventReceived`
              (`self.SpawnProjectiles` (`self.Projectile Target Location`) (`self.SocketTag`) _hitactor))))
        (:`OnCompleted`
          (`self.K2_EndAbility` :!label _label))
        (:`OnBlendOut`
          (goto _label))
        (:`OnInterrupted`
          (goto _label))
        (:`OnCancelled`
          (goto _label))))
    (:`HasNoTarget`
      (`self.K2_EndAbility`))))

(event `self.K2_OnEndAbility`
  (params (bWasCancelled :type Boolean))
  (message `CombatInterface.ClearActiveAbilityTag` (`self.GetAvatarActorFromActorInfo`)))