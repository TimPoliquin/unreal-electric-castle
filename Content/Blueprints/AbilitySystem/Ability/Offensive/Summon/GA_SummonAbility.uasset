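; Gameplay ability that has the avatar, apparently a Shaman, summon a group of minions.
; On activation it shuffles spawn locations, shows Niagara effects at each, plays the summon montage and waits for its attack event.
; A delayed loop then spawns random-class minions one by one, facing away from the summoner, with default controllers, registering each with the summon component.
; It ends when locations run out or the summoner dies.
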(event `self.K2_ActivateAbility`
  (bind _output_get (set `self.SpawnLocations` (`self.GetSpawnLocations`)))
  (`KismetArrayLibrary.Array_Shuffle` _output_get)
  (`self.ShowPreSpawningEffect` (`self.SpawnLocations`))
  (`AbilityTask_PlayMontageAndWait.CreatePlayMontageAndWaitProxy` "None" "/Game/Blueprints/Enemies/Shaman/Animations/AM_Shaman_Summon.AM_Shaman_Summon"
    (:`then`
      (`AbilityTask_WaitGameplayEvent.WaitGameplayEvent` (struct :`TagName` "Montage.Attack.0") null true
        (:`EventReceived`
          (if (< (`self.SpawnLocationIndex`) (`KismetArrayLibrary.Array_Length` (`self.SpawnLocations`))) :!label _label
            (`self.SpawnMinion`)
            (`/Engine/EditorBlueprintResources/StandardMacros.IncrementInt` (`self.SpawnLocationIndex`)
              (:`  `
                (`KismetSystemLibrary.Delay` 0.33)
                (bind _returnvalue (message `CombatInterface.IsDead` (`self.GetAvatarActorFromActorInfo`)))
                (if _returnvalue
                  (`self.K2_EndAbility`)
                  (else
                    (goto _label)))))
            (else
              (`self.K2_EndAbility`))))))))

(event `self.K2_OnEndAbility`
  (params (bWasCancelled :type Boolean))
  (set `self.SpawnLocationIndex` 0)
  (`KismetArrayLibrary.Array_Clear` (`self.SpawnLocations`)))

(fn `ShowPreSpawningEffect`
  (params (SpawnLocations :type "Array of Vector Structure"))
  (for _array_element SpawnLocations
    (`NiagaraFunctionLibrary.SpawnSystemAtLocation` (`self.SummonSystem`) _array_element)))

(fn `SpawnMinion`
  (returns (Minion :type "Pawn Object Reference"))
  (bind _returnvalue (+ (`|GetArrayItem` (`self.SpawnLocations`) (`self.SpawnLocationIndex`)) (0.0 0.0 70.0)))
  (bind _returnvalue_2 (`|SpawnActorFromClass` (`self.GetRandomSpawnClass`) (`KismetMathLibrary.MakeTransform` _returnvalue (`KismetMathLibrary.FindLookAtRotation` (`Actor.K2_GetActorLocation` (`self.GetAvatarActorFromActorInfo`)) _returnvalue)) "AlwaysSpawn" "MultiplyWithRoot" null null))
  (`Pawn.SpawnDefaultController` _returnvalue_2)
  (`self.Track Minion` _returnvalue_2)
  (return _returnvalue_2))

(fn `Track Minion`
  (params (Minion :type "Actor Object Reference"))
  (bind _returnvalue (message `SummoningActor.GetSummonComponent` (`self.GetAvatarActorFromActorInfo`)))
  (`/Engine/EditorBlueprintResources/StandardMacros.IsValid` _returnvalue
    (:`Is Valid`
      (`SummonComponent.AddMinion` _returnvalue (`local.Minion`)))))