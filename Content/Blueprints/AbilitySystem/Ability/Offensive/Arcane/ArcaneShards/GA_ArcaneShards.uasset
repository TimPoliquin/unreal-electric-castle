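; Gameplay ability for Arcane Shards, a targeted area spell that erupts a level-scaled number of shards around the cursor.
; It shows a magic circle, and on input press commits cost and generates ground points via a temporary BP_PointCollection.
; A cast montage event starts a looping timer that spawns shards sequentially, each applying radial damage with knockback and a GameplayCue.
; Cooldown commits after the last shard.
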(event `self.K2_ActivateAbility`
  (bind _returnvalue (`self.K2_CheckAbilityCost`))
  (if _returnvalue
    (`|ExecutionSequence`
      (:`then_0`
        (message `PlayerInterface.ShowMagicCircle` (`self.GetAvatarActorFromActorInfo`) null))
      (:`then_1`
        (`AbilityTask_WaitInputPress.WaitInputPress` false
          (:`OnPress`
            (bind _returnvalue_2 (`self.K2_CommitAbilityCost` false))
            (if _returnvalue_2
              (`|ExecutionSequence`
                (:`then_0`
                  ; Determine Shard Spawn Points
                  (bind (_asynctaskproxy _datahandle) (`TargetDataUnderMouse.CreateTargetDataUnderMouse` false)
                    (:`HasMouseTarget`
                      (bind (_returnvalue_bblockinghit _returnvalue_binitialoverlap _returnvalue_time _returnvalue_distance _returnvalue_location _returnvalue_impactpoint) (`GameplayStatics.BreakHitResult` (`AbilitySystemBlueprintLibrary.GetHitResultFromTargetData` _datahandle)))
                      (bind _returnvalue_3 (`|SpawnActorFromClass` "/Game/Blueprints/AbilitySystem/Ability/Offensive/Arcane/ArcaneShards/BP_PointCollection.BP_PointCollection_C" (`KismetMathLibrary.MakeTransform` _returnvalue_impactpoint) "Undefined" "MultiplyWithRoot" null null))
                      (set `self.PointCollection` _returnvalue_3)
                      (set `self.Ground Points` (`PointCollection.GetGroundPoints` (`self.PointCollection`) _returnvalue_impactpoint (`self.GetNumShards` (`self.GetAbilityLevel`)) 0.0))
                      (message `CombatInterface.UpdateFacingTarget` (`self.GetAvatarActorFromActorInfo`) _returnvalue_impactpoint))))
                (:`then_1`
                  ;[0.15 0 0.1467 0.5] Play Animation and Spawn Shards
                  (`AbilityTask_PlayMontageAndWait.CreatePlayMontageAndWaitProxy` "None" "/Game/Blueprints/Aura/Animations/AM_Player_Cast_ArcaneShards.AM_Player_Cast_ArcaneShards" 1.0 "None" false
                    (:`then`
                      (`AbilityTask_WaitGameplayEvent.WaitGameplayEvent` (struct :`TagName` "Event.Montage.ArcaneShards") null true
                        (:`EventReceived`
                          (bind _returnvalue_4 (`KismetSystemLibrary.K2_SetTimerDelegate` (delegate `SpawnShard_Event`) (`self.ShardSpawnDeltaTime`) true))
                          (set `self.Spawn Timer` _returnvalue_4)
                          (message `PlayerInterface.HideMagicCircle` (`self.GetAvatarActorFromActorInfo`))
                          (`self.SpawnShard_Event`)))))))
              (else
                (`self.K2_EndAbility`)))))))
    (else
      (`self.K2_EndAbility`))))

(event `SpawnShard_Event`
  ;[0.15 0 0.1467 0.5] Play Animation and Spawn Shards
  (`self.Execute_SpawnShard`))

(event `FinishAbility_Event`
  ; End Ability
  (message `PlayerInterface.HideMagicCircle` (`self.GetAvatarActorFromActorInfo`))
  (`self.K2_CommitAbilityCooldown` false)
  (`Actor.K2_DestroyActor` (`self.PointCollection`))
  (`self.K2_EndAbility`))

(fn `Execute_SpawnShard`
  (if (< (`self.SpawnedCount`) (`self.GetNumShards` (`self.GetAbilityLevel`)))
    (set `self.Shard Spawn Location` (`SceneComponent.K2_GetComponentLocation` (`|GetArrayItem` (`self.Ground Points`) (`self.SpawnedCount`))))
    (`|ExecutionSequence`
      (:`then_0`
        (`/Engine/EditorBlueprintResources/StandardMacros.IncrementInt` (`self.SpawnedCount`)))
      (:`then_1`
        ; Damage Enemies in the Impact Area
        (bind _hitenemies (`self.FindEnemiesWithinImpactRadius`))
        (for _array_element _hitenemies
          (bind _returnvalue (- (`Actor.K2_GetActorLocation` _array_element) (`self.Shard Spawn Location`)))
          (`ElectricCastleAbilitySystemLibrary.ApplyDamageEffect` (`self.MakeDamageEffectParamsFromClassDefaults` _array_element (`self.Shard Spawn Location`) true _returnvalue true _returnvalue true 35.0))))
      (:`then_2`
        ; Show Particle Effects (and broadcast)
        (`self.K2_ExecuteGameplayCueWithParams` (struct :`TagName` "GameplayCue.ArcaneShards") (`AbilitySystemBlueprintLibrary.MakeGameplayCueParameters` 0.0 0.0 (struct) (struct) (struct) (struct) (struct) (`self.Shard Spawn Location`)))))
    (else
      (`self.FinishAbility_Event`))))

(fn `FindEnemiesWithinImpactRadius`
  (returns (HitEnemies :type "Array of Actor Object Reference"))
  (bind _returnvalue (`self.GetAvatarActorFromActorInfo`))
  (bind (_damageconfig_damagetypetag _damageconfig_amount _damageconfig_debuffchance _damageconfig_debuffdamage _damageconfig_debufffrequency _damageconfig_debuffduration _damageconfig_deathimpulsemagnitude _damageconfig_knockbackforcemagnitude _damageconfig_knockbackchance _damageconfig_bisradialdamage _damageconfig_radialdamageinnerradius _damageconfig_radialdamageouterradius) (break `ElectricCastleDamageConfig` (`self.DamageConfig`)))
  (bind _returnvalue_2 (message `CombatInterface.GetTargetTagsToIgnore` _returnvalue))
  (bind _outoverlappingactors (`ElectricCastleAbilitySystemLibrary.GetLiveActorsWithinRadius` _returnvalue (`|MakeArray` _returnvalue) _returnvalue_2 (`self.Shard Spawn Location`) _damageconfig_radialdamageouterradius))
  (return _outoverlappingactors))