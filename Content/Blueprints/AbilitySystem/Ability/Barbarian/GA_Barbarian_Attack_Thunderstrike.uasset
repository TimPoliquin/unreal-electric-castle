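; Barbarian Thunderstrike gameplay ability: an area attack that damages targets around the avatar and applies the Thunderstruck effect to the caster.
; After committing, it plays the attack montage and waits for its Thunderstrike gameplay event.
; On authority, that event fires the lightning cue, then after a short delay a shockwave cue.
; The shockwave immediately triggers radial damage at the avatar's location, the self-applied effect and EndAbility.
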(event `self.K2_ActivateAbility`
  (bind _returnvalue (`self.K2_CommitAbility`))
  (if _returnvalue
    (`AbilityTask_PlayMontageAndWait.CreatePlayMontageAndWaitProxy` "None" "/Game/MetaHumans/MHC_Barbarian/Anim/Combat/AM_Barbarian_Attack_Thunderstrike.AM_Barbarian_Attack_Thunderstrike"
      (:`then`
        (`AbilityTask_WaitGameplayEvent.WaitGameplayEvent` (struct :`TagName` "Event.Montage.Barbarian.Thunderstrike") null true
          (:`EventReceived`
            (`self.Lightning Cue`)))))))

(event `Damage Enemies in Range`
  (bind _returnvalue (`Actor.K2_GetActorLocation` (`self.GetAvatarActorFromActorInfo`)))
  (`self.K2_HasAuthority`
    (:`True`
      (`self.DamageTargets` (`self.GetTargetsAtImpactLocation` _returnvalue 250.0) _returnvalue (`BlueprintGameplayTagLibrary.MakeLiteralGameplayTag` (struct :`TagName` "Event.Montage.Barbarian.Thunderstrike")))
      (`ElectricCastleAbilitySystemLibrary.ApplyBasicGameplayEffect` (`self.GetAvatarActorFromActorInfo`) "/Game/Blueprints/AbilitySystem/GameplayEffects/Barbarian/GE_Barbarian_Thunderstruck.GE_Barbarian_Thunderstruck_C" (`self.GetAbilityLevel`))
      (`self.K2_EndAbility`))))

(event `Lightning Cue`
  (bind _returnvalue (`self.GetAbilityLevel`))
  (`self.K2_HasAuthority`
    (:`True`
      (`self.K2_ExecuteGameplayCueWithParams` (struct :`TagName` "GameplayCue.Barbarian.Thunderstrike") (`AbilitySystemBlueprintLibrary.MakeGameplayCueParameters` 0.0 0.0 (struct) (struct) (struct) (struct) (struct) (`Actor.K2_GetActorLocation` (`self.GetAvatarActorFromActorInfo`)) (0.0 0.0 0.0) null (`self.GetAvatarActorFromActorInfo`) null null _returnvalue _returnvalue))
      (`KismetSystemLibrary.Delay` 0.1)
      (`self.Shockwave`))))

(event `Shockwave`
  (bind _returnvalue (`self.GetAbilityLevel`))
  (`self.K2_ExecuteGameplayCueWithParams` (struct :`TagName` "GameplayCue.Barbarian.Shockwave") (`AbilitySystemBlueprintLibrary.MakeGameplayCueParameters` 0.0 0.0 (struct) (struct) (struct) (struct) (struct) (`Actor.K2_GetActorLocation` (`self.GetAvatarActorFromActorInfo`)) (0.0 0.0 0.0) null (`self.GetAvatarActorFromActorInfo`) null null _returnvalue _returnvalue))
  (`self.Damage Enemies in Range`))